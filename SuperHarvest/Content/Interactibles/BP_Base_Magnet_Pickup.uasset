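; Base magnet pickup item that spins, bounces to a random nearby spot on spawn, and despawns after a timed lifetime.
; StartAttraction, queued until the bounce finishes, runs a timer that lerps the mesh toward the player using a random offset curve and a scale curve.
; DestroyAndAddItem passes ItemInfo to the instigator with a sound, while InventoryFullStopMoving halts attraction, restores scale and height, and resets lifetime.
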(event Custom|DestroyAndAddItem
  (params (Instigator :type Top%20Down%20Character%20Object%20Reference))
  ;[1 1 1] destroy and add item
  (Class|BPIMagnetOverlap|OnPickupMagnetItem(Message) Instigator (Variables|Default|GetItemInfo))
  (Audio|PlaySound2D "/Game/SFX/cue_plop.cue_plop")
  (Variables|Default|SetIsMoving? false)
  (Actor|DestroyActor))

(event Custom|StartAttraction
  ;[1 1 1] Start Attraction
  (if (Variables|Default|GetBounceComplete?)
    (Variables|Default|SetQueueMagnet? false)
    (Variables|Default|SetIsMoving? true)
    (Variables|Default|SetCurveIndexToUse (Math|Random|RandomIntegerinRange 0 4))
    (Utilities|Time|SetTimerbyEvent (delegate Custom|ContinueMoving) (Variables|Default|GetTime) (Variables|Default|GetIsMoving?))
    (else
      (Variables|Default|SetQueueMagnet? true))))

(event Custom|ContinueMoving
  ;[1 1 1] Translate over time
  (if (Variables|Default|GetIsMoving?)
    (Variables|Default|SetTimePassed (+ (Variables|Default|GetTime) (Variables|Default|GetTimePassed)))
    (bind _astop_down_character (Utilities|Casting|CastToTopDownCharacter (Game|GetPlayerCharacter 0)))
    (Transformation|SetWorldLocation (Variables|Default|GetStaticMesh) (Math|Vector|Lerp(Vector) (Transformation|GetWorldLocation (Variables|Default|GetStaticMesh)) (+ (Math|Vector|MakeVector (.X (Math|Vector|BreakVector (Transformation|GetActorLocation _astop_down_character))) (.Y (Math|Vector|BreakVector (Transformation|GetActorLocation _astop_down_character))) (- (.Z (Math|Vector|BreakVector (Transformation|GetActorLocation _astop_down_character))) 5e+01)) (Math|Curves|GetVectorValue (Utilities|Array|Get(acopy) (Variables|Default|GetCurves_Translate) (Variables|Default|GetCurveIndexToUse)) (Variables|Default|GetTimePassed))) 0.05) false false)
    ;[1 1 1] Scale over time
    (if (Variables|Default|GetIsMoving?)
      (Transformation|SetWorldScale3D (Variables|Default|GetStaticMesh) (Math|Curves|GetVectorValue (Variables|Default|GetCurves_Scale) (Variables|Default|GetTimePassed))))))

(event Custom|CheckTime
  ;[1 1 1] DespawnTimer
  (Variables|Default|SetTimeAlive (+ (Variables|Default|GetTimeAlive) 1.0))
  (if (>= (Variables|Default|GetTimeAlive) 2e+01)
    (Actor|DestroyActor)))

(event Custom|DespawnTimer
  ;[1 1 1] DespawnTimer
  (Utilities|Time|SetTimerbyEvent (delegate Custom|CheckTime) 1.0 true))

(event Custom|ChangeScaleAndLocation
  (bind _staticmesh (Variables|Default|GetStaticMesh))
  (bind _staticmesh_2 (Variables|Default|GetStaticMesh))
  (bind _staticmesh_3 (Variables|Default|GetStaticMesh))
  (bind _returnvalue (Transformation|GetWorldLocation _staticmesh_2))
  (bind _returnvalue_2 (Transformation|GetWorldLocation _staticmesh_3))
  (bind _returnvalue_3 (Transformation|GetWorldScale _staticmesh))
  (bind (_x _y _z) (Math|Vector|BreakVector _returnvalue))
  (bind (_x_2 _y_2) (Math|Vector|BreakVector _returnvalue_2))
  (bind (_x_3 _y_3 _z_2) (Math|Vector|BreakVector _returnvalue_3))
  ;[1 1 1] Reset Scale And Location Z
  ;[1 1 1] Reset Scale over Time
  (if (> (.X (Math|Vector|BreakVector (Transformation|GetWorldScale (Variables|Default|GetStaticMesh)))) 0.97)
    (Variables|Default|SetScaleIsLessThanOne? false)
    (Transformation|SetWorldScale3D (Variables|Default|GetStaticMesh) "1.000000,1.000000,1.000000")
    (else
      (Transformation|SetWorldScale3D (Variables|Default|GetStaticMesh) (Math|Vector|MakeVector (+ _x_3 0.01) (+ _y_3 0.01) (+ _z_2 0.01)))))
  ;[1 1 1] Reset Z Location
  (if (> (.Z (Math|Vector|BreakVector (Transformation|GetWorldLocation (Variables|Default|GetStaticMesh)))) 1.0)
    (Transformation|SetWorldLocation (Variables|Default|GetStaticMesh) (Math|Vector|MakeVector _x _y (- _z 1.0)) false false)
    (else
      (Variables|Default|SetLocationZIsMoreThanZero? false)
      (Transformation|SetWorldLocation (Variables|Default|GetStaticMesh) (Math|Vector|MakeVector _x_2 _y_2 0.0) false false))))

(event Custom|ResetMeshScale
  ;[1 1 1] Reset Scale And Location Z
  (Variables|Default|SetScaleIsLessThanOne? true)
  (Variables|Default|SetLocationZIsMoreThanZero? true)
  (Utilities|Time|SetTimerbyEvent (delegate Custom|ChangeScaleAndLocation) 0.01 (or (Variables|Default|GetScaleIsLessThanOne?) (Variables|Default|GetLocationZIsMoreThanZero?))))

(event Custom|InventoryFullStopMoving
  ;[1 1 1] stop move on full inventory
  (Variables|Default|SetIsMoving? false)
  (CallFunction|ResetMeshScale)
  (Variables|Default|SetTimeAlive 0.0))

(event EventTick
  (params (DeltaSeconds :type Float%20%28single-precision%29))
  ;[1 1 1] Rotate item on tick
  (Transformation|AddActorLocalRotation (Math|Rotator|MakeRotator 0.0 0.0 (* DeltaSeconds 8e+01)) false false))

(event EventBeginPlay
  ;[1 1 1] initial bounce
  (Variables|Default|SetBounceComplete? false)
  (Variables|Default|SetStartLocation (Transformation|GetWorldLocation (Variables|Default|GetStaticMesh)))
  (Variables|Default|SetGoalLocation (+ (Variables|Default|GetStartLocation) (Math|Vector|MakeVector (Math|Random|RandomFloatinRange -2e+02 2e+02) (Math|Random|RandomFloatinRange -2e+02 2e+02) 0.0)))
  (bind (_direction _alpha _bounce) (Timeline|SpawnBounce PlayFromStart)
    (:Update
      (Transformation|SetWorldLocation (Variables|Default|GetStaticMesh) (Math|Vector|Lerp(Vector) (Variables|Default|GetStartLocation) (+ (Variables|Default|GetGoalLocation) _bounce) _alpha) false false))
    (:Finished
      (Variables|Default|SetBounceComplete? true)
      (if (Variables|Default|GetQueueMagnet?)
        (CallFunction|StartAttraction)))))

(fn ConstructionScript
  (Transformation|AddActorLocalRotation (Math|Rotator|MakeRotator 0.0 0.0 (Math|Random|RandomFloatinRange 0.0 3.6e+02)) false false)
  (CallFunction|DespawnTimer))