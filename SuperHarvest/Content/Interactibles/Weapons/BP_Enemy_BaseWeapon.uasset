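; Base enemy ranged weapon that fires projectiles, configured by a WeaponInfo data table row looked up by ID.
; Fire spawns the row's projectile at ProjectileSpawnPoint with the owning AI's pawn as instigator, then holds an internal cooldown scaled by attack rate.
; Construction fills CurrentAmmo from magazine size, but Fire never checks or consumes it.
; Muzzle VFX and sound nodes are disconnected, noted as also handled in MainChar for replication.
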(event Custom|Fire
  (bind _returnvalue (Components|GetOwner))
  (bind _projectilespawnpoint (Variables|Default|GetProjectileSpawnPoint))
  (bind _returnvalue_2 (Transformation|GetWorldTransform _projectilespawnpoint))
  ;[1 1 1] Fire
  (bind _returnvalue_3 (Utilities|GetDataTableRow "/Game/Interactibles/WeaponInfo.WeaponInfo" (Variables|Default|GetID))
    (:then
      (Variables|Default|SetWeaponInfo _returnvalue_3)
      (if (not (Variables|Default|GetOnInternalCooldown))
        (Utilities|FlowControl|Sequence
          (:then_0
            (Game|SpawnActorfromClass (.RangedProjectile (Utilities|Struct|BreakFWeaponInfo (Variables|Default|GetWeaponInfo))) (Math|Transform|MakeTransform (.location _returnvalue_2) (.rotation _returnvalue_2) "1,1,1") "AlwaysSpawn" _returnvalue (.Lifetime (Utilities|Struct|BreakFWeaponInfo (Variables|Default|GetWeaponInfo))) (Pawn|GetControlledPawn (AI|GetAIController _returnvalue))))
          (:then_1
            (Variables|Default|SetOnInternalCooldown true)
            (Utilities|FlowControl|Delay (/ 0.8 (.AttacksPerSecond (Utilities|Struct|BreakFWeaponInfo (Variables|Default|GetWeaponInfo)))))
            (Variables|Default|SetOnInternalCooldown false)))))))

(fn ConstructionScript
  (|CallParentFunction)
  (bind _returnvalue (Utilities|GetDataTableRow "/Game/Interactibles/WeaponInfo.WeaponInfo" (Variables|Default|GetID))
    (:then
      (Variables|Default|SetCurrentAmmo (.MagazineSize (Utilities|Struct|BreakFWeaponInfo _returnvalue))))
    (:RowNotFound
      (Development|PrintString "Error row not found1"))))