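; Base weapon actor for the top-down character, handling ranged firing, ammo and reloading from a WeaponInfo data struct.
; Fire is blocked while Reloading, reloads on an empty magazine, or spends a round to spawn a damage-carrying projectile with VFX and sound at the owner's spawn point.
; Reload calls the owning character's Reload, plays a sound and refills ammo immediately; this Blueprint never sets the Reloading flag.
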(event EventBeginPlay)

(event Collision|EventActorBeginOverlap
  (params (OtherActor :type Actor%20Object%20Reference)))

(event EventTick
  (params (DeltaSeconds :type Float%20%28single-precision%29)))

(fn ConstructionScript
  (|CallParentFunction)
  (Variables|Default|SetCurrentAmmo (.magazinesize (Variables|Default|GetWeaponInfo))))

(fn Fire
  (bind _weaponinfo (Variables|Default|GetWeaponInfo))
  (if (not (Variables|Default|GetReloading))
    (if (<= (Variables|Default|GetCurrentAmmo) 0)
      (CallFunction|Reload)
      (else
        (Variables|Default|SetCurrentAmmo (- (Variables|Default|GetCurrentAmmo) 1))
        (bind _astop_down_character (Utilities|Casting|CastToTopDownCharacter (Components|GetOwner)))
        (bind _returnvalue (Game|SpawnActorfromClass (.rangedprojectile _weaponinfo) (Math|Transform|MakeTransform (.location (Transformation|GetWorldTransform (Variables|BP_BaseWeapon_C|GetProjectileSpawnPoint (Variables|/Game/Blueprints/TopDownCharacter.TopDownCharacter_C|GetWeapon _astop_down_character)))) (.rotation (Transformation|GetWorldTransform (Variables|BP_BaseWeapon_C|GetProjectileSpawnPoint (Variables|/Game/Blueprints/TopDownCharacter.TopDownCharacter_C|GetWeapon _astop_down_character)))) "1,1,1") "AlwaysSpawn" _astop_down_character (.lifetime _weaponinfo) _astop_down_character))
        (Variables|/Game/Blueprints/Projectiles/projectile_main.projectile_main_C|Setdamage _returnvalue (.damage _weaponinfo))
        (Effects|SpawnEmitteratLocation (.attackvfx _weaponinfo) (.location (Transformation|GetWorldTransform (Variables|BP_BaseWeapon_C|GetProjectileSpawnPoint (Variables|/Game/Blueprints/TopDownCharacter.TopDownCharacter_C|GetWeapon _astop_down_character)))) (.rotation (Transformation|GetWorldTransform (Variables|BP_BaseWeapon_C|GetProjectileSpawnPoint (Variables|/Game/Blueprints/TopDownCharacter.TopDownCharacter_C|GetWeapon _astop_down_character)))))
        (Audio|PlaySoundatLocation (.attacksfx _weaponinfo) (.location (Transformation|GetWorldTransform (Variables|BP_BaseWeapon_C|GetProjectileSpawnPoint (Variables|/Game/Blueprints/TopDownCharacter.TopDownCharacter_C|GetWeapon _astop_down_character)))) "0, 0, 0" 1.0 1.0 0.0 0 0 0)))))

(fn Reload
  (bind _weaponinfo (Variables|Default|GetWeaponInfo))
  (bind _astop_down_character (Utilities|Casting|CastToTopDownCharacter (Components|GetOwner)))
  (Default|Reload _astop_down_character)
  (Audio|PlaySoundatLocation (.reloadsfx _weaponinfo) (.location (Transformation|GetWorldTransform (Variables|BP_BaseWeapon_C|GetProjectileSpawnPoint (Variables|/Game/Blueprints/TopDownCharacter.TopDownCharacter_C|GetWeapon _astop_down_character)))) "0, 0, 0" 1.0 1.0 0.0 0 0 0)
  (Variables|Default|SetCurrentAmmo (.magazinesize _weaponinfo)))