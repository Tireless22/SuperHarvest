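; Enemy projectile actor that damages the player character on overlap and expires after a set lifetime.
; Overlaps on its collision component are filtered to actors that implement BPI_DamageableActor and whose class is exactly TopDownCharacter.
; A hit prints a debug message, destroys the projectile, then applies damage credited to the owner's AI controller and spawns an ArrowHit emitter at the victim's location.
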(event OnComponentBeginOverlap(ProjectileCollision)
  (params (OverlappedComponent :type Primitive%20Component%20Object%20Reference) (OtherActor :type Actor%20Object%20Reference) (OtherComp :type Primitive%20Component%20Object%20Reference) (OtherBodyIndex :type Integer) (bFromSweep :type Boolean) (SweepResult :type Hit%20Result%20Structure%20%28by%20ref%29))
  (bind _self self)
  (if (Utilities|DoesObjectImplementInterface OtherActor "/Game/Blueprints/BPI_DamageableActor.BPI_DamageableActor_C")
    (if (== (Utilities|GetClass OtherActor) "/Game/Blueprints/TopDownCharacter.TopDownCharacter_C")
      ;[1 1 1] Character Hit
      (Development|PrintString "Player Hit!" true true "(R=1.000000,G=0.034584,B=0.000000,A=1.000000)")
      (Actor|DestroyActor _self)
      (Game|Damage|ApplyDamage OtherActor (Variables|Default|Getdamage) (AI|GetAIController (Components|GetOwner)) _self)
      (Effects|SpawnEmitteratLocation "/Game/VFX/ArrowHit.ArrowHit" (Transformation|GetActorLocation OtherActor)))))

(event EventBeginPlay
  (Actor|SetLifeSpan (Variables|Default|GetLifeTime)))

(fn ConstructionScript
  (|CallParentFunction))