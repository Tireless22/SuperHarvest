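; Small projectile Blueprint that adds a stretch effect to its mesh on spawn, on top of the parent class's behavior.
; BeginPlay calls the parent, caches the mesh's world scale, then plays the StartScaling timeline.
; Each timeline update lerps the relative scale from that cached value toward a version elongated mostly along X and slightly widened along Y, leaving Z unchanged.
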(event EventBeginPlay
  (bind _projectilemesh (Variables|Default|GetProjectileMesh))
  ;[1 1 1] StartScaling, for effect
  (|CallParentFunction)
  (Variables|Default|SetNewVar_0_0 (Transformation|GetWorldScale _projectilemesh))
  (bind _newtrack_0 (Timeline|StartScaling PlayFromStart)
    (:Update
      (Transformation|SetRelativeScale3D _projectilemesh (Math|Vector|Lerp(Vector) (Variables|Default|GetNewVar_0_0) (Math|Vector|MakeVector (* (.X (Math|Vector|BreakVector (Variables|Default|GetNewVar_0_0))) 6.0) (* (.Y (Math|Vector|BreakVector (Variables|Default|GetNewVar_0_0))) 1.5) (.Z (Math|Vector|BreakVector (Variables|Default|GetNewVar_0_0)))) _newtrack_0)))))

(fn ConstructionScript
  (|CallParentFunction))