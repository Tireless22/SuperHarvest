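; Projectile actor that shrinks over its lifetime and destroys itself when that time runs out.
; Tick interpolates scale toward near zero at a constant rate derived from LifeTime.
; Collision overlap with the player only destroys the projectile and spawns a stone-chip effect at the player, with no damage applied.
; A SootEnemy overlap calls its TakeDamage through a DoOnce, leaving any projectile cleanup outside this Blueprint.
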(event OnComponentBeginOverlap(ProjectileCollision)
  (params (OverlappedComponent :type Primitive%20Component%20Object%20Reference) (OtherActor :type Actor%20Object%20Reference) (OtherComp :type Primitive%20Component%20Object%20Reference) (OtherBodyIndex :type Integer) (bFromSweep :type Boolean) (SweepResult :type Hit%20Result%20Structure%20%28by%20ref%29))
  (bind _returnvalue (Game|Player|GetPlayerPawn 0))
  (if (== OtherActor _returnvalue)
    ;[1 1 1] Player Hit
    (Development|PrintString "Player Hit!" true true "(R=1.000000,G=0.034584,B=0.000000,A=1.000000)")
    (Actor|DestroyActor self)
    (Effects|SpawnEmitteratLocation "/Game/Assets/VFX/stone_chips_big.stone_chips_big" (Transformation|GetActorLocation _returnvalue))
    (else
      ;[1 1 1] Soot Enemy Hit
      (bind _assoot_enemy (Utilities|Casting|CastToSootEnemy OtherActor)
        (:then
          (Utilities|FlowControl|DoOnce false
            (:Completed
              (Default|TakeDamage _assoot_enemy (Variables|Components|Getdamage) SweepResult OtherActor self)
              (Development|PrintString "Soot Hit!"))))
        (:CastFailed
          (Development|PrintString "ProjectileHit: Not enemy soot or MainChar"))))))

(event EventBeginPlay
  ;[1 1 1] Projectile Lifetime
  (Utilities|FlowControl|Delay (Variables|Default|GetLifeTime))
  (Actor|DestroyActor))

(event Collision|EventActorBeginOverlap
  (params (OtherActor :type Actor%20Object%20Reference)))

(event EventTick
  (params (DeltaSeconds :type Float%20%28single-precision%29))
  ;[1 1 1] Scale over lifetime
  (Transformation|SetActorScale3D (Math|Interpolation|VInterptoConstant (Transformation|GetWorldScale (Variables|Default|GetProjectileCollision)) "0.010000,0.010000,0.010000" DeltaSeconds (/ 1.0 (Variables|Default|GetLifeTime)))))

(fn ConstructionScript)