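; Base choppable tree Blueprint that takes hits, falls away from the player and yields BP_log pickups from trunk and stump.
; TreeHit shakes the tree until health drops to 100, then a timeline tips TreeBase along one axis chosen from player yaw, spawning a log.
; Further hits shake the remaining TreeTrunk until it yields another log and is destroyed.
; SetTransparencyOn fades in translucent dynamic materials, and a looping timer restores opaque ones when the player leaves.
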(event Custom|TreeHit
  (params (Damage :type Integer))
  (Variables|Default|SetHealth (- (Variables|Default|GetHealth) Damage))
  (if (<= (Variables|Default|GetHealth) 100)
    (if (Variables|Default|GetIsBaseDying?)
      (if (<= (Variables|Default|GetHealth) 0)
        (Audio|PlaySound2D "/Game/SFX/BaseSounds/wood_chop_01.wood_chop_01" 1.0 (Math|Random|RandomFloatinRange 0.8 1.0) 0.0 0 0)
        (Game|SpawnActorfromClass "/Game/Interactibles/Magnet_Items/BP_log.BP_log_C" (Math|Transform|MakeTransform (Transformation|GetWorldLocation (Variables|Default|GetTreeTrunk))) "Undefined" 0 0)
        (Actor|DestroyActor)
        (else
          (CallFunction|PlayTrunkShake)))
      (else
        (Variables|Default|SetIsBaseDying? true)
        (Audio|PlaySound2D "/Game/SFX/BaseSounds/wood_chop_01.wood_chop_01" 1.0 (Math|Random|RandomFloatinRange 0.8 1.0) 0.0 0 0)
        (Audio|PlaySound2D "/Game/SFX/BaseSounds/tree_falling_01.tree_falling_01" 1.0 (Math|Random|RandomFloatinRange 0.8 1.0) 0.0 0 0)
        ;[1 1 1] Tree Base dying and falling
        (bind _astop_down_character (Utilities|Casting|CastToTopDownCharacter (Game|GetPlayerCharacter 0))
          (:then
            (bind _output_get (Variables|Default|SetZFallDirection (.Yaw (Math|Rotator|BreakRotator (Math|Rotator|FindLookatRotation (Transformation|GetWorldLocation (Variables|/Script/Engine.Character|GetMesh _astop_down_character)) (Transformation|GetWorldLocation (Variables|Default|GetTreeBase)))))))
            (Development|PrintString (Utilities|String|ToString(Float) _output_get) true true "(R=0.000000,G=0.660000,B=1.000000,A=1.000000)" 5.0)
            (if (Math|Float|InRange(Float) (Variables|Default|GetZFallDirection) -45.0 45.0)
              (Variables|Default|SetNegativeY? true)
              (Variables|Default|SetImpactLocationOffset "0.000000,150.000000, 0")
              (bind (_direction _rotation90positive _rotation90negative) (Timeline|TreeFalling PlayFromStart)
                (:Update
                  (if (Variables|Default|GetNegativeX?)
                    (Transformation|SetWorldRotation (Variables|Default|GetTreeBase) (Math|Rotator|MakeRotator _rotation90negative 0.0 0.0) false false)
                    (elif (Variables|Default|GetNegativeY?)
                      (Transformation|SetWorldRotation (Variables|Default|GetTreeBase) (Math|Rotator|MakeRotator 0.0 _rotation90negative 0.0) false false)
                      (elif (Variables|Default|GetPositiveX?)
                        (Transformation|SetWorldRotation (Variables|Default|GetTreeBase) (Math|Rotator|MakeRotator _rotation90positive 0.0 0.0) false false)
                        (elif (Variables|Default|GetPositiveY?)
                          (Transformation|SetWorldRotation (Variables|Default|GetTreeBase) (Math|Rotator|MakeRotator 0.0 _rotation90positive 0.0) false false)
                          (else
                            (Development|PrintString "error")))))))
                (:Finished
                  (Audio|PlaySound2D "/Game/SFX/BaseSounds/tree_hit_ground_01.tree_hit_ground_01" 1.0 1.0 0.0 0 0)
                  (Effects|SpawnEmitteratLocation "/Game/VFX/leaf_cloud_small.leaf_cloud_small" (+ (Transformation|GetWorldLocation (Variables|Default|GetTreeTrunk)) (Variables|Default|GetImpactLocationOffset)))
                  (Game|SpawnActorfromClass "/Game/Interactibles/Magnet_Items/BP_log.BP_log_C" (Math|Transform|MakeTransform (+ (Transformation|GetWorldLocation (Variables|Default|GetTreeTrunk)) (Variables|Default|GetImpactLocationOffset))) "Undefined" 0 0)
                  (Components|DestroyComponent (Variables|Default|GetTreeBase))))
              (elif (Math|Float|InRange(Float) (Variables|Default|GetZFallDirection) -135.0 -45.0)
                (Variables|Default|SetNegativeX? true)
                (Variables|Default|SetImpactLocationOffset "0,-150.000000, 0")
                (Timeline|TreeFalling PlayFromStart)
                (elif (Math|Float|InRange(Float) (Variables|Default|GetZFallDirection) 45.0 135.0)
                  (Variables|Default|SetPositiveX? true)
                  (Variables|Default|SetImpactLocationOffset "-150.000000, 0, 0")
                  (Timeline|TreeFalling PlayFromStart)
                  (elif (Math|Float|InRange(Float) (Variables|Default|GetZFallDirection) 135.0 1.8e+02)
                    (Variables|Default|SetPositiveY? true :!label _label)
                    (Variables|Default|SetImpactLocationOffset "150.000000, 0, 0")
                    (Timeline|TreeFalling PlayFromStart)
                    (elif (Math|Float|InRange(Float) (Variables|Default|GetZFallDirection) -1.8e+02 -135.0)
                      (goto _label)
                      (else
                        (Development|PrintString "ERRORRR"))))))))
          (:CastFailed
            (Development|PrintString "castfail")))))
    (else
      (CallFunction|PlayBaseShake))))

(event Custom|PlayBaseShake
  (bind _treebase (Variables|Default|GetTreeBase))
  (bind _returnvalue (Transformation|GetWorldRotation _treebase))
  (bind (_roll _pitch _yaw) (Math|Rotator|BreakRotator _returnvalue))
  ;[1 1 1] PlayShake and sound when hit
  (Audio|PlaySound2D "/Game/SFX/BaseSounds/wood_chop_01.wood_chop_01" 1.0 (Math|Random|RandomFloatinRange 0.8 1.0) 0.0 0 0)
  (CallFunction|SpawnLeafEmitters)
  (Variables|Default|SetStartRotation (Transformation|GetWorldRotation (Variables|Default|GetTreeBase)))
  (bind _xyshake (Timeline|Shake PlayFromStart)
    (:Update
      (Transformation|SetWorldRotation (Variables|Default|GetTreeBase) (Math|Rotator|MakeRotator (+ _roll (.X (Math|Vector|BreakVector _xyshake))) (+ _pitch (.Y (Math|Vector|BreakVector _xyshake))) _yaw) false false))))

(event Custom|CheckDistanceToPawn
  (bind _treebase (Variables|Default|GetTreeBase))
  (if (Variables|Default|GetIsBaseDying?)
    (Utilities|Time|ClearandInvalidateTimerbyHandle (stale Custom|SetTransparencyOn _returnvalue_4) :!label _label)
    (bind _alpha (Timeline|FadeIn PlayFromStart)
      (:Update
        (Variables|Default|SetOpacityValue _alpha)
        (Rendering|Material|SetScalarParameterValue (Variables|Default|GetBrownMaterialRef) "Opacity" (Variables|Default|GetOpacityValue) :!class /Script/Engine.MaterialInstanceDynamic)
        (Rendering|Material|SetScalarParameterValue (Variables|Default|GetGreenMaterialRef) "Opacity" (Variables|Default|GetOpacityValue) :!class /Script/Engine.MaterialInstanceDynamic)
        (Rendering|Material|SetScalarParameterValue (Variables|Default|GetGreenLeafRef) "Opacity" (Variables|Default|GetOpacityValue) :!class /Script/Engine.MaterialInstanceDynamic))
      (:Finished
        (Rendering|Material|SetMaterial _treebase 0 "/Game/Assets/Materials/Flat_Brown.Flat_Brown")
        (Rendering|Material|SetMaterial _treebase 1 "/Game/Assets/Materials/Flat_Green.Flat_Green")
        (Rendering|Material|SetMaterial _treebase 2 "/Game/Assets/Meshes/Foliage/materials/m_leaf_01.m_leaf_01")
        (Variables|Default|SetTransparencyOn? false)))
    (else
      (bind _astop_down_character (Utilities|Casting|CastToTopDownCharacter (Game|GetPlayerCharacter 0)))
      (if (> (Math|Vector|VectorLength (- (Transformation|GetWorldLocation (Variables|Default|GetTreeBase)) (Transformation|GetWorldLocation (Variables|/Script/Engine.Character|GetMesh _astop_down_character)))) 2e+02)
        (goto _label)))))

(event Custom|SetTransparencyOn
  (bind _treebase (Variables|Default|GetTreeBase))
  (bind _treebase_2 (Variables|Default|GetTreeBase))
  (if (not (Variables|Default|GetTransparencyOn?))
    (if (not (Variables|Default|GetIsBaseDying?))
      (Variables|Default|SetTransparencyOn? true)
      (bind _returnvalue (Rendering|Material|CreateDynamicMaterialInstance "/Game/Assets/Meshes/Foliage/materials/m_leaf_transparent.m_leaf_transparent" "None" :!class /Script/Engine.KismetMaterialLibrary))
      (Variables|Default|SetGreenLeafRef _returnvalue)
      (bind _returnvalue_2 (Rendering|Material|CreateDynamicMaterialInstance "/Game/Assets/Materials/Flat_Transparent_Brown.Flat_Transparent_Brown" "None" :!class /Script/Engine.KismetMaterialLibrary))
      (Variables|Default|SetBrownMaterialRef _returnvalue_2)
      (bind _returnvalue_3 (Rendering|Material|CreateDynamicMaterialInstance "/Game/Assets/Materials/Flat_Transparent_green.Flat_Transparent_green" "None" :!class /Script/Engine.KismetMaterialLibrary))
      (Variables|Default|SetGreenMaterialRef _returnvalue_3)
      (Rendering|Material|SetMaterial _treebase_2 0 (Variables|Default|GetBrownMaterialRef))
      (Rendering|Material|SetMaterial _treebase_2 1 (Variables|Default|GetGreenMaterialRef))
      (Rendering|Material|SetMaterial _treebase_2 2 (Variables|Default|GetGreenLeafRef))
      (bind _alpha (Timeline|FadeOut PlayFromStart)
        (:Update
          (Variables|Default|SetOpacityValue _alpha)
          (Rendering|Material|SetScalarParameterValue (Variables|Default|GetBrownMaterialRef) "Opacity" (Variables|Default|GetOpacityValue) :!class /Script/Engine.MaterialInstanceDynamic)
          (Rendering|Material|SetScalarParameterValue (Variables|Default|GetGreenMaterialRef) "Opacity" (Variables|Default|GetOpacityValue) :!class /Script/Engine.MaterialInstanceDynamic)
          (Rendering|Material|SetScalarParameterValue (Variables|Default|GetGreenLeafRef) "Opacity" (Variables|Default|GetOpacityValue) :!class /Script/Engine.MaterialInstanceDynamic))
        (:Finished
          (if (Variables|Default|GetIsBaseDying?)
            (Utilities|Time|ClearandInvalidateTimerbyHandle (stale _returnvalue_4))
            (bind _alpha_2 (Timeline|FadeIn PlayFromStart)
              (:Update
                (Variables|Default|SetOpacityValue _alpha_2)
                (Rendering|Material|SetScalarParameterValue (Variables|Default|GetBrownMaterialRef) "Opacity" (Variables|Default|GetOpacityValue) :!class /Script/Engine.MaterialInstanceDynamic)
                (Rendering|Material|SetScalarParameterValue (Variables|Default|GetGreenMaterialRef) "Opacity" (Variables|Default|GetOpacityValue) :!class /Script/Engine.MaterialInstanceDynamic)
                (Rendering|Material|SetScalarParameterValue (Variables|Default|GetGreenLeafRef) "Opacity" (Variables|Default|GetOpacityValue) :!class /Script/Engine.MaterialInstanceDynamic))
              (:Finished
                (Rendering|Material|SetMaterial _treebase 0 "/Game/Assets/Materials/Flat_Brown.Flat_Brown")
                (Rendering|Material|SetMaterial _treebase 1 "/Game/Assets/Materials/Flat_Green.Flat_Green")
                (Rendering|Material|SetMaterial _treebase 2 "/Game/Assets/Meshes/Foliage/materials/m_leaf_01.m_leaf_01")
                (Variables|Default|SetTransparencyOn? false)))
            (else
              (bind _returnvalue_4 (Utilities|Time|SetTimerbyEvent (delegate Custom|CheckDistanceToPawn) 0.2 true)))))))))

(event Custom|PlayTrunkShake
  (bind _treetrunk (Variables|Default|GetTreeTrunk))
  (bind _returnvalue (Transformation|GetWorldRotation _treetrunk))
  (bind (_roll _pitch _yaw) (Math|Rotator|BreakRotator _returnvalue))
  ;[1 1 1] play trunk shake
  (Audio|PlaySound2D "/Game/SFX/BaseSounds/wood_chop_01.wood_chop_01" 1.0 (Math|Random|RandomFloatinRange 0.8 1.0) 0.0 0 0)
  (Variables|Default|SetStartRotation (Transformation|GetWorldRotation (Variables|Default|GetTreeTrunk)))
  (bind _xyshake (Timeline|Timeline_0 PlayFromStart)
    (:Update
      (Transformation|SetWorldRotation (Variables|Default|GetTreeTrunk) (Math|Rotator|MakeRotator (+ _roll (.X (Math|Vector|BreakVector _xyshake))) (+ _pitch (.Y (Math|Vector|BreakVector _xyshake))) _yaw) false false))))

(fn ConstructionScript
  (Variables|Default|SetRandomRotation (Math|Random|RandomFloatinRange 0.0 3.6e+02))
  (Transformation|SetWorldRotation (Variables|Default|GetTreeBase) "0, 0, 0" false false)
  (Transformation|SetWorldRotation (Variables|Default|GetTreeTrunk) "0, 0, 0" false false))

(fn SpawnLeafEmitters
  (Effects|SpawnEmitteratLocation "/Game/VFX/leaf_fall_small.leaf_fall_small" (Transformation|GetWorldLocation (Variables|Default|GetArrow)))
  (Effects|SpawnEmitteratLocation "/Game/VFX/leaf_fall_small.leaf_fall_small" (Transformation|GetWorldLocation (Variables|Default|GetArrow1)))
  (Effects|SpawnEmitteratLocation "/Game/VFX/leaf_fall_small.leaf_fall_small" (Transformation|GetWorldLocation (Variables|Default|GetArrow2)))
  (return))