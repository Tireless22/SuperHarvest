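; Actor that randomly scatters actors, configured by the Spawn_Area_Forest data table, inside a box area at BeginPlay.
; Each row resizes the box and sets the class, count and footprint to place at random points with random yaw.
; Randomized downward line traces around each point reject spots based on hits and physical surface type (SurfaceType2 passes).
; Failed placements extend the spawn loop until the row's MaxTries is reached; traces draw debug lines.
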(event EventBeginPlay
  (bind _box (Variables|Default|GetBox))
  (bind (_origin _boxextent) (Collision|GetComponentBounds _box))
  (bind _returnvalue (Math|Random|RandomPointinBoundingBox _origin _boxextent))
  (bind (_x _y) (Math|Vector|BreakVector _returnvalue))
  (bind _outrownames (DataTable|GetDataTableRowNames "/Game/Blueprints/Spawn_Area_Forest.Spawn_Area_Forest"))
  (Variables|Default|SetRowNamesArray _outrownames)
  (for _array_element (Variables|Default|GetRowNamesArray)
    (bind _returnvalue_2 (Utilities|GetDataTableRow "/Game/Blueprints/Spawn_Area_Forest.Spawn_Area_Forest" _array_element)
      (:then
        (Utilities|Array|Add (Variables|Default|GetSpawnArray) _returnvalue_2))
      (:RowNotFound
        (Development|PrintString "Error row not foudn!" true true "(R=0.031194,G=0.990053,B=1.000000,A=1.000000)"))))
  (for _array_element_2 (Variables|Default|GetSpawnArray)
    (Variables|Default|SetSpawnInfoRef _array_element_2)
    (Variables|Default|SetMaxTries (.MaxTries (Utilities|Struct|BreakSpawnInfo (Variables|Default|GetSpawnInfoRef))))
    (Variables|Default|SetItemsToSpawn (.ItemsAmount (Utilities|Struct|BreakSpawnInfo (Variables|Default|GetSpawnInfoRef))))
    (Variables|Default|SetTimesTried 0)
    (Components|Box|SetBoxExtent (Variables|Default|GetBox) (Math|Vector|MakeVector (.BoxExtent (Utilities|Struct|BreakSpawnInfo (Variables|Default|GetSpawnInfoRef))) (.BoxExtent (Utilities|Struct|BreakSpawnInfo (Variables|Default|GetSpawnInfoRef))) 1e+02) true)
    (for _index (range 0 (- (Variables|Default|GetItemsToSpawn) 1))
      (Variables|Default|SetLocRef (Math|Vector|MakeVector _x _y 0.0))
      (Variables|Default|SetAreaClear? true)
      (Utilities|FlowControl|ForLoopwithBreak 0 (Utilities|Struct|BreakSpawnInfo (Variables|Default|GetSpawnInfoRef)) :!label _label
        (:LoopBody
          (bind (_outhit _returnvalue_3) (Collision|LineTraceForObjects (Math|Vector|MakeVector (.X (Math|Vector|BreakVector (Math|Random|RandomPointinBoundingBox (Variables|Default|GetLocRef) (Math|Vector|MakeVector (Utilities|Struct|BreakSpawnInfo (Variables|Default|GetSpawnInfoRef)) (Utilities|Struct|BreakSpawnInfo (Variables|Default|GetSpawnInfoRef)) (Utilities|Struct|BreakSpawnInfo (Variables|Default|GetSpawnInfoRef)))))) (.Y (Math|Vector|BreakVector (Math|Random|RandomPointinBoundingBox (Variables|Default|GetLocRef) (Math|Vector|MakeVector (Utilities|Struct|BreakSpawnInfo (Variables|Default|GetSpawnInfoRef)) (Utilities|Struct|BreakSpawnInfo (Variables|Default|GetSpawnInfoRef)) (Utilities|Struct|BreakSpawnInfo (Variables|Default|GetSpawnInfoRef)))))) 5e+02) (Math|Random|RandomPointinBoundingBox (Variables|Default|GetLocRef) (Math|Vector|MakeVector (Utilities|Struct|BreakSpawnInfo (Variables|Default|GetSpawnInfoRef)) (Utilities|Struct|BreakSpawnInfo (Variables|Default|GetSpawnInfoRef)) (Utilities|Struct|BreakSpawnInfo (Variables|Default|GetSpawnInfoRef)))) (Utilities|Array|MakeArray "ObjectTypeQuery1" "ObjectTypeQuery2" "ObjectTypeQuery3" "ObjectTypeQuery4" "ObjectTypeQuery5" "ObjectTypeQuery6" "ObjectTypeQuery7" "ObjectTypeQuery8" "ObjectTypeQuery9") false 0 "ForDuration"))
          (if (== (.PhysMat (Collision|BreakHitResult _outhit)) 0)
            (if _returnvalue_3
              (Variables|Default|SetAreaClear? false :!label _label_2)
              (goto _label Break))
            (elif (not (Utilities|Enum|Equal(Enum) (Variables|/Script/Engine.PhysicalMaterial|GetSurfaceType (.PhysMat (Collision|BreakHitResult _outhit))) "SurfaceType2"))
              (goto _label_2))))
        (:Completed
          (if (Variables|Default|GetAreaClear?)
            (Game|SpawnActorfromClass (Utilities|Struct|BreakSpawnInfo (Variables|Default|GetSpawnInfoRef)) (Math|Transform|MakeTransform (Variables|Default|GetLocRef) (Math|Rotator|MakeRotator 0.0 0.0 (Math|Random|RandomFloatinRange 0.0 3.6e+02))) "Undefined" 0 0)
            (Math|Integer|IncrementInt (Variables|Default|GetTimesTried))
            (else
              ;[1 1 1] failed to spawn actor increasing forloop if not max nr of tries reached
              (Math|Integer|IncrementInt (Variables|Default|GetTimesTried)
                (:%20%20
                  (if (not (>= (Variables|Default|GetTimesTried) (Variables|Default|GetMaxTries)))
                    (Math|Integer|IncrementInt (Variables|Default|GetItemsToSpawn))))))))))))

(fn ConstructionScript)