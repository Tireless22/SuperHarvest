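; Plowable earth area that turns dig locations into furrow meshes on a 100-unit square grid centred on origin.
; DigMesh snaps the location to a cell in a flattened array and spawns an Earth_Mesh if it is undug.
; CheckNeighbours picks one of four mesh types from left/right Y-axis neighbours and updates theirs to connect.
; The last-index check is hard-coded to 99, and the boundary helper is unused here.
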(event Custom|DigMesh
  (params (Location :type Vector))
  (bind _halfwidthunits (Variables|Default|GetHalfWidthUnits))
  (Variables|Default|SetInitialDigLocation Location)
  (Variables|Default|SetRoundedDigLocation (Math|Vector|MakeVector (- (Math|Conversions|ToFloat(Integer) (* (.ReturnValue (Math|Float|Division(WholeandRemainder) (+ (.X (Math|Vector|BreakVector (Variables|Default|GetInitialDigLocation))) (Math|Conversions|ToFloat(Integer) _halfwidthunits)) 1e+02)) 100)) (Math|Conversions|ToFloat(Integer) (Variables|Default|GetHalfWidthUnits))) (- (Math|Conversions|ToFloat(Integer) (* (.ReturnValue (Math|Float|Division(WholeandRemainder) (+ (.Y (Math|Vector|BreakVector (Variables|Default|GetInitialDigLocation))) (Math|Conversions|ToFloat(Integer) _halfwidthunits)) 1e+02)) 100)) (Math|Conversions|ToFloat(Integer) (Variables|Default|GetHalfWidthUnits))) 1.0))
  (Variables|Default|SetDigX (.ReturnValue (Math|Float|Division(WholeandRemainder) (+ (.X (Math|Vector|BreakVector (Variables|Default|GetInitialDigLocation))) (Math|Conversions|ToFloat(Integer) _halfwidthunits)) 1e+02)))
  (Variables|Default|SetDigY (.ReturnValue (Math|Float|Division(WholeandRemainder) (+ (.Y (Math|Vector|BreakVector (Variables|Default|GetInitialDigLocation))) (Math|Conversions|ToFloat(Integer) _halfwidthunits)) 1e+02)))
  (Development|PrintString (Utilities|String|BuildString(Integer) "X =  " "" (Variables|Default|GetDigX)))
  (Development|PrintString (Utilities|String|BuildString(Integer) "Y =  " "" (Variables|Default|GetDigY)))
  (Variables|Default|SetMeshIndexToChange (- (+ (* (Variables|Default|GetDigX) (Variables|Default|GetColumnLength)) (Variables|Default|GetColumnLength)) (- (Variables|Default|GetColumnLength) (Variables|Default|GetDigY))))
  (if (== (Utilities|Array|Get(acopy) (Variables|Default|GetStaticMeshTypeInfo) (Variables|Default|GetMeshIndexToChange)) -1)
    (CallFunction|CheckNeighbours)
    (else
      (Development|PrintString "allready dug here"))))

(event EventBeginPlay
  (bind _halfwidthunits (Variables|Default|GetHalfWidthUnits))
  (bind _returnvalue (/ _halfwidthunits 100))
  (bind _returnvalue_2 (* _returnvalue 2))
  (Variables|Default|SetMyLocation (Transformation|GetWorldLocation (Variables|Default|GetDefaultSceneRoot)))
  (Variables|Default|SetColumnLength _returnvalue_2)
  (Variables|Default|SetNumberOfGrids (* _returnvalue_2 _returnvalue_2))
  (for _index (range 0 (- (Variables|Default|GetNumberOfGrids) 1))
    (Utilities|Array|Add (Variables|Default|GetStaticMeshTypeInfo) -1)
    (Utilities|Array|Add (Variables|Default|GetEarthMeshArray) 0))
  (Development|PrintString (Utilities|String|ToString(Integer) (Utilities|Array|Length (Variables|Default|GetStaticMeshTypeInfo))))
  (Development|PrintString (Utilities|String|ToString(Integer) (Utilities|Array|Length (Variables|Default|GetEarthMeshArray)))))

(fn ConstructionScript)

(fn IsLocationWithinBoundary?
  (params (InitialDigLocation :type Vector))
  (bind (_x _y) (Math|Vector|BreakVector InitialDigLocation))
  (bind _halfwidthunits (Variables|Default|GetHalfWidthUnits))
  (bind _halfwidthunits_2 (Variables|Default|GetHalfWidthUnits))
  (bind _returnvalue (Math|Conversions|ToFloat(Integer) _halfwidthunits_2))
  (bind _returnvalue_2 (Math|Conversions|ToFloat(Integer) _halfwidthunits))
  (bind _returnvalue_3 (+ _x _returnvalue_2))
  (bind _returnvalue_4 (+ _y _returnvalue))
  (if (< _returnvalue_3 0.0)
    (LocalVariables|SetInside? false :!label _label)
    (elif (> _returnvalue_3 (* (Math|Conversions|ToFloat(Integer) (Variables|Default|GetHalfWidthUnits)) 2.0))
      (goto _label)
      (elif (< _returnvalue_4 0.0)
        (goto _label)
        (elif (> _returnvalue_4 (* (Math|Conversions|ToFloat(Integer) (Variables|Default|GetHalfWidthUnits)) 2.0))
          (goto _label)
          (else
            (LocalVariables|SetInside? true))))))
  (return (LocalVariables|GetInside?)))

(fn ChangeTypeonNeighbourSide
  (params (ChangeRightMesh :type Boolean))
  (bind _meshindextochange (Variables|Default|GetMeshIndexToChange))
  (bind _meshindextochange_2 (Variables|Default|GetMeshIndexToChange))
  (bind _returnvalue (- _meshindextochange 1))
  (bind _returnvalue_2 (+ _meshindextochange_2 1))
  (LocalVariables|SetChangeRightSide?Ref ChangeRightMesh)
  (if (LocalVariables|GetChangeRightSide?Ref)
    (LocalVariables|SetTypeInfo (Utilities|Array|Get(acopy) (Variables|Default|GetStaticMeshTypeInfo) _returnvalue_2))
    (LocalVariables|SetMeshIndexRef _returnvalue_2)
    (else
      (LocalVariables|SetTypeInfo (Utilities|Array|Get(acopy) (Variables|Default|GetStaticMeshTypeInfo) _returnvalue))
      (LocalVariables|SetMeshIndexRef _returnvalue)))
  (if (LocalVariables|GetChangeRightSide?Ref)
    (Development|PrintString "change my right side")
    (switch int (LocalVariables|GetTypeInfo)
      (:1
        (LocalVariables|SetChangedMeshInfo? false :!label _label))
      (:2
        (LocalVariables|SetTypeInfo 1)
        (LocalVariables|SetChangedMeshInfo? true :!label _label_2))
      (:3
        (goto _label))
      (:4
        (LocalVariables|SetTypeInfo 3)
        (goto _label_2)))
    (else
      (Development|PrintString "change my left side")
      ;[1 1 1] change my left side
      (switch int (LocalVariables|GetTypeInfo)
        (:1
          (LocalVariables|SetChangedMeshInfo? false :!label _label_3))
        (:2
          (goto _label_3))
        (:3
          (LocalVariables|SetTypeInfo 1)
          (LocalVariables|SetChangedMeshInfo? true :!label _label_4))
        (:4
          (LocalVariables|SetTypeInfo 2)
          (goto _label_4)))))
  (if (LocalVariables|GetChangedMeshInfo?)
    (Utilities|Array|SetArrayElem (Variables|Default|GetStaticMeshTypeInfo) (LocalVariables|GetMeshIndexRef) (LocalVariables|GetTypeInfo))
    (Default|SetMyMesh (Utilities|Array|Get(acopy) (Variables|Default|GetEarthMeshArray) (LocalVariables|GetMeshIndexRef)) (LocalVariables|GetTypeInfo))
    (else
      (Development|PrintString "mesh info remained the same")))
  (return))

(fn CheckNeighbours
  (if (== (Variables|Default|GetMeshIndexToChange) 0)
    ;[1 1 1] checking if mesh exists on left and/or right side
    (LocalVariables|SetMeshExistToMyLeft? false :!label _label)
    (elif (== (Utilities|Array|Get(acopy) (Variables|Default|GetStaticMeshTypeInfo) (- (Variables|Default|GetMeshIndexToChange) 1)) -1)
      (goto _label)
      (else
        (LocalVariables|SetMeshExistToMyLeft? true))))
  (if (== (Variables|Default|GetMeshIndexToChange) 99)
    (LocalVariables|SetMeshExistsToMyRight? false :!label _label_2)
    (elif (== (Utilities|Array|Get(acopy) (Variables|Default|GetStaticMeshTypeInfo) (+ (Variables|Default|GetMeshIndexToChange) 1)) -1)
      (goto _label_2)
      (else
        (LocalVariables|SetMeshExistsToMyRight? true))))
  ;[1 1 1] checking if we are on the far end of right or left. If we are to either side we override previous added item
  (if (== (Variables|Default|GetDigY) (- (Variables|Default|GetColumnLength) 1))
    (Development|PrintString "Im on the far right side")
    (LocalVariables|SetMeshExistsToMyRight? false))
  (if (== (Variables|Default|GetDigY) 0)
    (Development|PrintString "Im on the far left side ")
    (LocalVariables|SetMeshExistToMyLeft? false))
  (if (LocalVariables|GetMeshExistToMyLeft?)
    ;[1 1 1] editing surrounding meshes if they exist
    (CallFunction|ChangeTypeonNeighbourSide false))
  (if (LocalVariables|GetMeshExistsToMyRight?)
    (CallFunction|ChangeTypeonNeighbourSide true))
  (if (LocalVariables|GetMeshExistToMyLeft?)
    (if (LocalVariables|GetMeshExistsToMyRight?)
      (Variables|Default|SetMeshTypeInfo 1)
      (else
        (Variables|Default|SetMeshTypeInfo 3)))
    (elif (LocalVariables|GetMeshExistsToMyRight?)
      (Variables|Default|SetMeshTypeInfo 2)
      (else
        (Variables|Default|SetMeshTypeInfo 4))))
  (Utilities|Array|SetArrayElem (Variables|Default|GetStaticMeshTypeInfo) (Variables|Default|GetMeshIndexToChange) (Variables|Default|GetMeshTypeInfo))
  (Development|PrintString (Utilities|String|BuildString(Integer) "new mesh index is: " "" (Variables|Default|GetMeshIndexToChange)))
  (bind _returnvalue (Game|SpawnActorfromClass "/Game/Blueprints/Earth_Mesh.Earth_Mesh_C" (Math|Transform|MakeTransform (Variables|Default|GetRoundedDigLocation)) "Undefined" 0 0))
  (Utilities|Array|SetArrayElem (Variables|Default|GetEarthMeshArray) (Variables|Default|GetMeshIndexToChange) _returnvalue)
  (Default|SetMyMesh _returnvalue (Variables|Default|GetMeshTypeInfo)))