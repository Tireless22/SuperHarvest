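; Legacy networked Soot enemy Character that chases and attacks players with a sword and a server-spawned, attached shield.
; A looping half-second timer handles targeting, SimpleMoveToActor chasing, attacks, distance-based health-bar fading and a shield stance driven by player facing and reloading.
; Timelines blend the stance and walk speed; damage flashes the material and raises the shield, while death multicasts ragdoll and data-table loot drops.
; Old shield-hit and projectile-deflection logic remains disconnected.
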(event OnComponentHit(ShieldCol)
  (params (HitComponent :type Primitive%20Component%20Object%20Reference) (OtherActor :type Actor%20Object%20Reference) (OtherComp :type Primitive%20Component%20Object%20Reference) (NormalImpulse :type Vector :default "0, 0, 0") (Hit :type Hit%20Result%20Structure%20%28by%20ref%29))
  ;[1 1 1] Projectile Hit Shield?
)

(event Custom|ShieldUp
  ;[1 1 1] Go Into Shield Stance on Damage + Enable Shield Colision
  (if (and (== (Variables|Default|GetShieldUp?) 0.0) (!= (Variables|/Game/Interactibles/Weapons/Shields/Soot_Shield.Soot_Shield_C|GetShieldDurability (Variables|Default|GetShield)) 0.0))
    (Utilities|FlowControl|DoOnce false :!label _label
      (:Completed
        (bind _time (Timeline|lerpTime PlayFromStart)
          (:Update
            (Utilities|FlowControl|Sequence
              (:then_0
                (Variables|Default|SetShieldUp? (Math|Float|Lerp 0.0 1.0 _time)))
              (:then_1
                (Variables|/Script/Engine.CharacterMovementComponent|SetMaxWalkSpeed (Variables|Character|GetCharacterMovement) (Math|Float|Lerp (Variables|Default|GetStartRunSpeed) (Variables|Default|GetStartWalkSpeed) _time)))))
          (:Finished
            (Utilities|FlowControl|Sequence
              (:then_0
                (Utilities|FlowControl|RetriggerableDelay 1e+01)
                (if (Variables|Default|GetLooking%20At)
                  (CallFunction|ShieldDown)))
              (:then_1
                (goto _label Reset))
              (:then_2
                (Collision|SetCollisionEnabled (Variables|/Game/Interactibles/Weapons/Shields/Soot_Shield.Soot_Shield_C|GetShieldCol (Variables|Default|GetShield)) "QueryOnly")))))))))

(event Custom|MainEvents
  (bind _returnvalue (Game|GetPlayerController 0))
  (bind _topdowncharacterreference (Variables|Default|GetTopDownCharacterReference))
  (bind _topdowncharacterreference_2 (Variables|Default|GetTopDownCharacterReference))
  (bind _returnvalue_2 (Pawn|GetControlledPawn _returnvalue))
  ;[1 1 1] AI
  (Utilities|FlowControl|Sequence
    (:then_1
      ;[1 1 1] Select Target
      (if (== (Variables|Default|GetTopDownCharacterReference) 0)
        (bind _outactors (Actor|GetAllActorsOfClass "/Game/Blueprints/TopDownCharacter.TopDownCharacter_C"))
        (for _array_element _outactors
          (Variables|Default|SetCurrentDistanceTo (Transformation|GetDistanceTo _array_element self))
          (if (<= (Transformation|GetDistanceTo _array_element self) (Variables|Default|GetCurrentDistanceTo))
            (CallFunction|ServerSetTarget _array_element)))
        (elif (>= (Transformation|GetDistanceTo (Variables|Default|GetTopDownCharacterReference) self) 3e+02)
          (Utilities|FlowControl|DoOnce false :!label _label
            (:Completed
              (Development|PrintString "TOO FAR AWAY FOR AGGRO")
              (CallFunction|ServerUnSetTarget)))
          (else
            (goto _label Reset)))))
    (:then_2
      ;[1 1 1] MoveToActor
      (Utilities|IsValid _topdowncharacterreference
        (:Is%20Valid
          (if (not (<= (Transformation|GetDistanceTo _topdowncharacterreference) 1.5e+02))
            (CallFunction|ServerSetMove)))))
    (:then_3
      ;[1 1 1] Attack when within 100units. Wants to be moved to BlackBoard
      (Utilities|IsValid _topdowncharacterreference_2
        (:Is%20Valid
          (if (<= (Transformation|GetDistanceTo _topdowncharacterreference_2) 1e+02) :!label _label_2
            (Variables|Default|SetAttack true)
            (Utilities|FlowControl|Delay (Variables|Default|GetAttackAnimLength))
            (Variables|Default|SetAttack false)
            (goto _label_2)
            (else
              (Variables|Default|SetAttack false))))))
    (:then_4
      ;[1 1 1] Shield Up / Down on LookAt
      (Utilities|IsValid (Variables|Default|GetTopDownCharacterReference)
        (:Is%20Valid
          (if (and (>= (* (Math|Vector|DotProduct (Math|Vector|GetForwardVector (Math|Rotator|FindLookatRotation (Transformation|GetActorLocation) (Transformation|GetActorLocation (Variables|Default|GetTopDownCharacterReference)))) (Math|Vector|GetForwardVector (Transformation|GetWorldRotation (Variables|/Script/Engine.Character|GetCapsuleComponent (Variables|Default|GetTopDownCharacterReference))))) -1.0) 0.8) (!= (Variables|/Game/Interactibles/Weapons/Shields/Soot_Shield.Soot_Shield_C|GetShieldDurability (Variables|Default|GetShield)) 0.0))
            (Utilities|FlowControl|DoOnce false :!label _label_3
              (:Completed
                (Variables|Default|SetLooking%20At true :!label _label_4)
                (CallFunction|ShieldUp)
                (goto _label_5 Reset)))
            (else
              (Utilities|FlowControl|DoOnce false :!label _label_5
                (:Completed
                  (Variables|Default|SetLooking%20At false :!label _label_6)
                  (CallFunction|ShieldDown)
                  (goto _label_3 Reset))))))))
    (:then_5
      ;[1 1 1] Shield Up / Down on Player Reload
      (Utilities|IsValid (Variables|Default|GetTopDownCharacterReference)
        (:Is%20Valid
          (if (!= (Variables|/Game/Interactibles/Weapons/Shields/Soot_Shield.Soot_Shield_C|GetShieldDurability (Variables|Default|GetShield)) 0.0)
            (if (and (Variables|Default|GetLooking%20At) (Variables|/Game/Blueprints/TopDownCharacter.TopDownCharacter_C|GetReloading? (Variables|Default|GetTopDownCharacterReference)))
              (Utilities|FlowControl|Sequence
                (:then_0
                  (Utilities|FlowControl|DoOnce false :!label _label_7
                    (:Completed
                      (Utilities|FlowControl|Delay 0.5)
                      (goto _label_6))))
                (:then_1
                  (goto _label_8 Reset)))
              (else
                (Utilities|FlowControl|Sequence
                  (:then_0
                    (Utilities|FlowControl|DoOnce true :!label _label_8
                      (:Completed
                        (Utilities|FlowControl|Delay 0.5)
                        (goto _label_4))))
                  (:then_1
                    (goto _label_7 Reset)))))))))
    (:then_6
      ;[1 1 1] UI Fade (Doesn't need to be networked, right?)
      (Utilities|IsValid _returnvalue_2
        (:Is%20Valid
          (if (<= (Transformation|GetDistanceTo _returnvalue_2) 6e+02)
            (if (not (Variables|Default|GetCalledFadeOut?))
              (Variables|Default|SetCalledFadeOut? true)
              (CallFunction|FadeUI true))
            (elif (Variables|Default|GetCalledFadeOut?)
              (Variables|Default|SetCalledFadeOut? false)
              (CallFunction|FadeUI false))))))))

(event Custom|MultiCast_ShieldTakeDamage
  (params (Damage :type Float%20%28single-precision%29) (Target :type Soot%20Shield%20Object%20Reference))
  (Variables|/Game/Interactibles/Weapons/Shields/Soot_Shield.Soot_Shield_C|SetShieldDurability Target Damage)
  (Development|PrintString "d1")
  (CallFunction|UpdateUIShield))

(event Custom|Server_UpdateUI
  (CallFunction|MultiCastUpdateUI))

(event Custom|MultiCast_UpdateUI
  (CallFunction|UpdateUIShield))

(event Custom|Final%20Shield%20Down
  ;[1 1 1] Go Into Shield Stance on Damage + Enable Shield Colision
  (Variables|Default|SetShieldUp? 0.0)
  (Variables|/Script/Engine.CharacterMovementComponent|SetMaxWalkSpeed (Variables|Character|GetCharacterMovement) 475.0))

(event Custom|ShieldDown
  ;[1 1 1] Go Into Shield Stance on Damage + Enable Shield Colision
  (if (!= (Variables|/Game/Interactibles/Weapons/Shields/Soot_Shield.Soot_Shield_C|GetShieldDurability (Variables|Default|GetShield)) 0.0)
    (bind _time (Timeline|Timeline_0 PlayFromStart)
      (:Update
        (Utilities|FlowControl|Sequence
          (:then_0
            (Variables|Default|SetShieldUp? (Math|Float|Lerp 1.0 0.0 _time)))
          (:then_1
            (Variables|/Script/Engine.CharacterMovementComponent|SetMaxWalkSpeed (Variables|Character|GetCharacterMovement) (Math|Float|Lerp (Variables|Default|GetStartWalkSpeed) (Variables|Default|GetStartRunSpeed) _time)))
          (:then_2
            (Collision|SetCollisionEnabled (Variables|/Game/Interactibles/Weapons/Shields/Soot_Shield.Soot_Shield_C|GetShieldCol (Variables|Default|GetShield)) "NoCollision")))))))

(event Custom|Shield%20Damage%20Visibility
  ;[1 1 1] MOVED TO SHIELD ACTOR
)

(event Custom|Server_SetTarget
  (params (TopDownCharacterReference :type Top%20Down%20Character%20Object%20Reference))
  ;[1 1 1] Select Target
  (Variables|Default|SetTopDownCharacterReference TopDownCharacterReference))

(event Custom|Soot%20Enemy%20Damage%20Visibility
  (bind _mesh (Variables|Character|GetMesh))
  ;[1 1 1] Damage Shader Toggle
  (Rendering|Material|SetMaterial _mesh 4 "/Game/Assets/Materials/Emissive_Red.Emissive_Red")
  (Utilities|FlowControl|Delay 0.15)
  (Rendering|Material|SetMaterial _mesh 4 (Variables|Default|GetSootBodyColor)))

(event Custom|Server_SetMove
  ;[1 1 1] MoveToActor
  (AI|Navigation|SimpleMovetoActor (AI|GetAIController self) (Variables|Default|GetTopDownCharacterReference)))

(event Custom|Server_UnSetTarget
  ;[1 1 1] Select Target
  (Variables|Default|SetTopDownCharacterReference 0))

(event Custom|MultiCast_HitEffect
  ;[1 1 1] TakeDamage
  ;;[1 1 1] Set Shield Up on Damage
  (CallFunction|ShieldUp)
  (Effects|SpawnEmitteratLocation "/Game/VFX/leaf_fall_small.leaf_fall_small" (Transformation|GetActorLocation)) ; HitReaction Effect (Blood?)
  ;;[1 1 1] Update HP Text
  (CallFunction|UpdateUIHealth))

(event Custom|MultiCast_Death
  (bind _mesh (Variables|Character|GetMesh))
  (bind _shield (Variables|Default|GetShield))
  (bind _sword (Variables|Default|GetSword))
  (bind _shieldcol (Variables|/Game/Interactibles/Weapons/Shields/Soot_Shield.Soot_Shield_C|GetShieldCol _shield))
  ;[1 1 1] TakeDamage
  ;;[1 1 1] disable event loop
  (Utilities|Time|ClearandInvalidateTimerbyHandle (Variables|Default|GetMainTimerHandle))
  (Effects|SpawnEmitteratLocation "/Game/VFX/grass_straw_cloud_01.grass_straw_cloud_01" (Transformation|GetActorLocation))
  ;;[1 1 1] Death
  ;;;[1 1 1] Disable More! No Anim, No Ai
  (Pawn|Components|CharacterMovement|DisableMovement (Variables|Character|GetCharacterMovement))
  (Physics|SetSimulatePhysics _mesh true)
  (Collision|SetCollisionResponsetoChannel _mesh "ECC_Pawn" "ECR_Ignore")
  (Utilities|FlowControl|Sequence
    (:then_0
      (Transformation|DetachFromComponent (Variables|/Script/Engine.Actor|GetRootComponent (Variables|Default|GetShield)) "KeepWorld" "KeepWorld" "KeepWorld" true)
      (Collision|SetCollisionEnabled _shieldcol "PhysicsOnly")
      (Physics|SetSimulatePhysics _shieldcol true)
      (Collision|SetCollisionResponsetoChannel _shieldcol "ECC_Pawn" "ECR_Ignore"))
    (:then_1
      (Transformation|DetachFromComponent _sword "KeepWorld" "KeepWorld" "KeepWorld" true)
      (Collision|SetCollisionEnabled _sword "PhysicsOnly")
      (Physics|SetSimulatePhysics _sword true)
      (Collision|SetCollisionResponsetoChannel _sword "ECC_Pawn" "ECR_Ignore"))
    (:then_2
      (Components|Animation|SetAnimationMode (Variables|Character|GetMesh) "AnimationSingleNode"))
    (:then_3
      (Collision|SetCollisionEnabled (Variables|Collision|GetCapsuleComponent) "NoCollision"))
    (:then_4
      (CallFunction|SpawnLoot))
    (:then_5
      (Rendering|SetVisibility (Variables|Default|GetWidget) false false))
    (:then_6
      (Utilities|FlowControl|Delay 8.0)
      (Actor|DestroyActor))))

(event Custom|MultiCast_EventBeginPlay
  (params (Target :type Soot%20Shield%20Object%20Reference) (A :type Float%20%28single-precision%29))
  (CallFunction|UpdateUIShield))

(event Custom|Server_ShieldTakeDamage
  (params (Damage :type Float%20%28single-precision%29) (Target :type Soot%20Shield%20Object%20Reference))
  (CallFunction|MultiCastShieldTakeDamage Damage Target))

(event EventBeginPlay
  (bind _self self)
  ;[1 1 1] BeginPlay
  (Variables|Default|SetStartHealth (Variables|Default|GetHealth))
  (Variables|Default|SetStartRunSpeed (Variables|/Script/Engine.CharacterMovementComponent|GetMaxWalkSpeed (Variables|Character|GetCharacterMovement)))
  (Variables|Default|SetStartWalkSpeed 2e+02)
  (Variables|Default|SetSootBodyColor (Rendering|Material|GetMaterial (Variables|Character|GetMesh) 4))
  (CallFunction|UpdateUIHealth)
  (bind _returnvalue (Utilities|Time|SetTimerbyEvent (delegate Custom|MainEvents) 0.5 true))
  (Variables|Default|SetMainTimerHandle _returnvalue)
  (Networking|SwitchHasAuthority
    (:Authority
      (bind _returnvalue_2 (Game|SpawnActorfromClass "/Game/Interactibles/Weapons/Shields/Soot_Shield.Soot_Shield_C" (Transformation|GetActorTransform) "Undefined" _self _self))
      (bind _output_get (Variables|Default|SetShield _returnvalue_2))
      (Transformation|AttachComponentToComponent _output_get (Variables|Character|GetMesh) "LeftHand_ItemJoint" "SnapToTarget" "SnapToTarget" "SnapToTarget" false)
      (Collision|SetActorEnableCollision _output_get true)
      (Utilities|FlowControl|Delay 1.0)
      (CallFunction|MultiCastEventBeginPlay 0 0.0))))

(event EventShieldTakeDamage
  (params (Damage :type Float%20%28single-precision%29)))

(event Game|Damage|EventAnyDamage
  (params (Damage :type Float%20%28single-precision%29) (DamageType :type Damage%20Type%20Object%20Reference) (InstigatedBy :type Controller%20Object%20Reference) (DamageCauser :type Actor%20Object%20Reference))
  ;[1 1 1] TakeDamage
  (Variables|Default|SetHealth (- (Variables|Default|GetHealth) Damage))
  (CallFunction|SootEnemyDamageVisibility)
  (if (<= (Variables|Default|GetHealth) 0.0)
    (CallFunction|MultiCastDeath)
    (else
      (CallFunction|MultiCastHitEffect))))

(fn ConstructionScript)

(fn SpawnLoot
  (Development|PrintString "Rolling for loot!")
  (bind _outrownames (DataTable|GetDataTableRowNames "/Game/Interactibles/Soot_LootList.Soot_LootList"))
  (for _array_element _outrownames
    (bind _returnvalue (Utilities|GetDataTableRow "/Game/Interactibles/Soot_LootList.Soot_LootList" _array_element)
      (:then
        (LocalVariables|SetDropChance (.DropChance (Utilities|Struct|BreakLootList _returnvalue)))
        (LocalVariables|SetIDName (.ID (Utilities|Struct|BreakLootList _returnvalue)))
        (LocalVariables|SetMaxAmount (.MaxAmount (Utilities|Struct|BreakLootList _returnvalue)))
        (LocalVariables|SetClassRef (.ActorClass (Utilities|Struct|BreakLootList _returnvalue)))
        (LocalVariables|SetMinAmount (.MinAmount (Utilities|Struct|BreakLootList _returnvalue)))
        (if (Math|Float|InRange(Float) (Math|Random|RandomFloatinRange 0.0 1.0) 0.0 (LocalVariables|GetDropChance))
          (for _index (range (LocalVariables|GetMinAmount) (LocalVariables|GetMaxAmount))
            (bind _asbp_base_item (Utilities|Casting|CastToBP_BaseItemClass (LocalVariables|GetClassRef)))
            (Game|SpawnActorfromClass _asbp_base_item (Transformation|GetWorldTransform (Variables|Character|GetMesh)) "Undefined" 0 true false 0))
          (else
            (Development|PrintString "rolled for no loot" true true "(R=0.347548,G=0.000000,B=1.000000,A=1.000000)"))))
      (:RowNotFound
        (Development|PrintString "Error did not find row")))))

(fn UpdateUIHealth
  (bind _asui_health_bar (Utilities|Casting|CastToUI_HealthBar (UserInterface|GetUserWidgetObject (Variables|Default|GetWidget)))
    (:then
      (Variables|/Game/UI/UI_HealthBar.UI_HealthBar_C|SetHealthPercent _asui_health_bar (/ (Variables|Default|GetHealth) (Variables|Default|GetStartHealth))))
    (:CastFailed
      (Development|PrintString "castfail"))))

(fn UpdateUIShield
  (bind _shield (Variables|Default|GetShield))
  (bind _asui_health_bar (Utilities|Casting|CastToUI_HealthBar (UserInterface|GetUserWidgetObject (Variables|Default|GetWidget)))
    (:then
      (Variables|/Game/UI/UI_HealthBar.UI_HealthBar_C|SetShieldPercent _asui_health_bar (/ (Variables|/Game/Interactibles/Weapons/Shields/Soot_Shield.Soot_Shield_C|GetShieldStartDurability _shield) (Variables|/Game/Interactibles/Weapons/Shields/Soot_Shield.Soot_Shield_C|GetShieldDurability _shield))))
    (:CastFailed
      (Development|PrintString "cast fail 2"))))

(fn FadeUI
  (params (FadeOut? :type Boolean))
  (LocalVariables|SetRef FadeOut?)
  (bind _asui_health_bar (Utilities|Casting|CastToUI_HealthBar (UserInterface|GetUserWidgetObject (Variables|Default|GetWidget)))
    (:then
      (Default|SetStartFade _asui_health_bar (LocalVariables|GetRef)))
    (:CastFailed
      (Development|PrintString "castfail"))))