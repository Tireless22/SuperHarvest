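; Test Blueprint that procedurally builds a flat grid mesh on BeginPlay through a RuntimeMesh component.
; One loop steps column by column at GridWidth spacing to fill the vertex array, printing a warning on overrun.
; A second loop adds two triangles per cell using index offsets from ColumnLength.
; Only vertices and triangles feed the section, which gets a flat green material; normal, UV and tangent literals are unused.
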(event EventBeginPlay
  (bind _runtimemesh (Variables|Default|GetRuntimeMesh))
  (bind _columnlength (Variables|Default|GetColumnLength))
  (bind _columnlength_2 (Variables|Default|GetColumnLength))
  (Variables|Default|SetNumberOfVertices (/ (* (* (Variables|Default|GetColumnLength) (Variables|Default|GetRowLength)) 4) 2))
  (Variables|Default|SetVertexVectorRef "")
  (for _index (range 0 (- (Variables|Default|GetNumberOfVertices) 1))
    (if (Variables|Default|GetAddedFirst?)
      (if (>= (.Y (Math|Vector2D|BreakVector2D (Variables|Default|GetVertexVectorRef))) (Math|Conversions|ToFloat(Integer) (* (Variables|Default|GetGridWidth) (Variables|Default|GetColumnLength))))
        (if (>= (.X (Math|Vector2D|BreakVector2D (Variables|Default|GetVertexVectorRef))) (Math|Conversions|ToFloat(Integer) (* (Variables|Default|GetGridWidth) (Variables|Default|GetRowLength))))
          (Development|PrintString "Too many in forloop")
          (else
            (Variables|Default|SetVertexVectorRef (Math|Vector2D|MakeVector2D (+ (.X (Math|Vector2D|BreakVector2D (Variables|Default|GetVertexVectorRef))) (Math|Conversions|ToFloat(Integer) (Variables|Default|GetGridWidth))) 0.0))
            (Utilities|Array|Add (Variables|Default|GetVerticesArray) (Math|Vector|MakeVector (.X (Math|Vector2D|BreakVector2D (Variables|Default|GetVertexVectorRef))) (.Y (Math|Vector2D|BreakVector2D (Variables|Default|GetVertexVectorRef))) 0.0))))
        (else
          (Variables|Default|SetVertexVectorRef (Math|Vector2D|MakeVector2D (.X (Math|Vector2D|BreakVector2D (Variables|Default|GetVertexVectorRef))) (+ (.Y (Math|Vector2D|BreakVector2D (Variables|Default|GetVertexVectorRef))) (Math|Conversions|ToFloat(Integer) (Variables|Default|GetGridWidth)))))
          (Utilities|Array|Add (Variables|Default|GetVerticesArray) (Math|Vector|MakeVector (.X (Math|Vector2D|BreakVector2D (Variables|Default|GetVertexVectorRef))) (.Y (Math|Vector2D|BreakVector2D (Variables|Default|GetVertexVectorRef))) 0.0))))
      (else
        (Utilities|Array|Add (Variables|Default|GetVerticesArray) (Math|Vector|MakeVector (.X (Math|Vector2D|BreakVector2D (Variables|Default|GetVertexVectorRef))) (.Y (Math|Vector2D|BreakVector2D (Variables|Default|GetVertexVectorRef))) 0.0))
        (Variables|Default|SetAddedFirst? true))))
  (for _index_2 (range 0 (- (* (Variables|Default|GetColumnLength) (Variables|Default|GetRowLength)) 1))
    (Utilities|Array|Add (Variables|Default|GetTrianglesArray) _index_2)
    (Utilities|Array|Add (Variables|Default|GetTrianglesArray) (+ _index_2 1))
    (Utilities|Array|Add (Variables|Default|GetTrianglesArray) (+ _index_2 (* _columnlength_2 _columnlength_2)))
    (Utilities|Array|Add (Variables|Default|GetTrianglesArray) _index_2)
    (Utilities|Array|Add (Variables|Default|GetTrianglesArray) (+ _index_2 (* _columnlength _columnlength)))
    (Utilities|Array|Add (Variables|Default|GetTrianglesArray) (+ _index_2 (+ (Variables|Default|GetColumnLength) 1))))
  (Class|RuntimeMeshComponent|CreateMeshSectionBlueprint _runtimemesh 0 (Variables|Default|GetVerticesArray) (Variables|Default|GetTrianglesArray) 0 0 0 0 0 false false false "Average")
  (Rendering|Material|SetMaterial _runtimemesh 0 "/Game/Assets/Materials/Flat_Green.Flat_Green")
  (Utilities|FlowControl|Delay 2.0))

(fn ConstructionScript)