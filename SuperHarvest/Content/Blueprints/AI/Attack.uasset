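; Attack is a behavior tree task that checks whether the blackboard's target actor is player pawn 0.
; On a match it caches a TopDownChar cast once through a DoOnce and finishes successfully; otherwise it only prints a debug string and never calls FinishExecute.
; The logic that toggles an Attack flag over the animation length is disconnected, so the task performs no attack.
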(event EventReceiveExecuteAI
  (params (OwnerController :type AI%20Controller%20Object%20Reference) (ControlledPawn :type Pawn%20Object%20Reference))
  (if (== (Class|BTFunctionLibrary|GetBlackboardValueasObject (Variables|Default|GetTargetActorKey)) (Game|Player|GetPlayerPawn 0))
    (Utilities|FlowControl|Sequence
      (:then_0
        (Utilities|FlowControl|DoOnce false
          (:Completed
            (bind _topdowncharref (CallFunction|CasttoTopDownChar))
            (Variables|Default|SetTopDownReference _topdowncharref))))
      (:then_1
        (AI|BehaviorTree|FinishExecute true)))
    (else
      (Development|PrintString "Not Player Target ActorKey"))))