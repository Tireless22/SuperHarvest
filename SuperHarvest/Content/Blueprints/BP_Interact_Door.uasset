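; Interactable door that moves the TopDownCharacter to another level, either by streaming or by opening it by name.
; Trigger box tracks whether the player is in range, while a sphere fades the world interact button in and out.
; OpenDoor shows a loading screen, teleports and freezes the player, then swaps streamed levels and restores walking, or opens the level.
; An optional looping timer turns the widget toward the camera.
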(event OnComponentBeginOverlap(DoorTriggerBox)
  (params (OverlappedComponent :type Primitive%20Component%20Object%20Reference) (OtherActor :type Actor%20Object%20Reference) (OtherComp :type Primitive%20Component%20Object%20Reference) (OtherBodyIndex :type Integer) (bFromSweep :type Boolean) (SweepResult :type Hit%20Result%20Structure%20%28by%20ref%29))
  ;[1 1 1] On overlap set is in range
  (if (Utilities|Enum|Equal(Enum) (Utilities|GetDisplayName OtherActor) "TopDownCharacter")
    (Variables|Default|SetIsInRange? true)))

(event OnComponentEndOverlap(DoorTriggerBox)
  (params (OverlappedComponent :type Primitive%20Component%20Object%20Reference) (OtherActor :type Actor%20Object%20Reference) (OtherComp :type Primitive%20Component%20Object%20Reference) (OtherBodyIndex :type Integer))
  ;[1 1 1] On overlap set is in range
  (if (Utilities|Enum|Equal(Enum) (Utilities|GetDisplayName OtherActor) "TopDownCharacter")
    (Variables|Default|SetIsInRange? false)))

(event OnComponentBeginOverlap(WidgetSphere)
  (params (OverlappedComponent :type Primitive%20Component%20Object%20Reference) (OtherActor :type Actor%20Object%20Reference) (OtherComp :type Primitive%20Component%20Object%20Reference) (OtherBodyIndex :type Integer) (bFromSweep :type Boolean) (SweepResult :type Hit%20Result%20Structure%20%28by%20ref%29))
  ;[1 1 1] on overlap show interact
  (if (Utilities|Enum|Equal(Enum) (Utilities|GetDisplayName OtherActor) "TopDownCharacter")
    (bind _asui_world_interact_button (Utilities|Casting|CastToUI_WorldInteractButton (UserInterface|GetUserWidgetObject (Variables|Default|GetWidget))))
    (Default|Fadein _asui_world_interact_button)))

(event OnComponentEndOverlap(WidgetSphere)
  (params (OverlappedComponent :type Primitive%20Component%20Object%20Reference) (OtherActor :type Actor%20Object%20Reference) (OtherComp :type Primitive%20Component%20Object%20Reference) (OtherBodyIndex :type Integer))
  ;[1 1 1] on overlap show interact
  (if (Utilities|Enum|Equal(Enum) (Utilities|GetDisplayName OtherActor) "TopDownCharacter")
    (bind _asui_world_interact_button (Utilities|Casting|CastToUI_WorldInteractButton (UserInterface|GetUserWidgetObject (Variables|Default|GetWidget))))
    (Default|FadeOut _asui_world_interact_button)))

(event Custom|OpenDoor
  ;[1 1 1] Open Door Event
  (bind _returnvalue (UserInterface|CreateWidget "/Game/UI/UI_LoadingScreen.UI_LoadingScreen_C" (Game|GetPlayerController 0)))
  (Variables|Default|SetLoadingRef _returnvalue)
  (UserInterface|Viewport|AddtoViewport _returnvalue 0)
  (Utilities|FlowControl|Delay 1.0)
  (bind _astop_down_character (Utilities|Casting|CastToTopDownCharacter (Game|GetPlayerCharacter 0))
    (:then
      (Transformation|Teleport _astop_down_character (Transformation|GetWorldLocation (Variables|Default|GetPlayerNewPosition)) "0, 0, 0")
      (Pawn|Components|CharacterMovement|SetMovementMode (Variables|/Script/Engine.Character|GetCharacterMovement _astop_down_character) "MOVE_None" 0)
      (if (Variables|Default|GetLevelTravellingToIsStreamed?)
        ;[1 1 1] streamed level
        (Game|LoadStreamLevel(byName) (Variables|Default|GetLevelTravellingTo) true)
        (bind _astop_down_character_2 (Utilities|Casting|CastToTopDownCharacter (Game|GetPlayerCharacter 0))
          (:then
            (Pawn|Components|CharacterMovement|SetMovementMode (Variables|/Script/Engine.Character|GetCharacterMovement _astop_down_character_2) "MOVE_Walking" 0)
            (Default|FadeOutLoadingScreen (Variables|Default|GetLoadingRef))
            (Game|UnloadStreamLevel(byName) (Variables|Default|GetLevelComingFrom)))
          (:CastFailed
            (Development|PrintString "cast fail")))
        (else
          (Game|OpenLevel(byName) (Variables|Default|GetLevelTravellingTo)))))
    (:CastFailed
      (Development|PrintString "cast fail"))))

(event Custom|AlignToCamera
  ;[1 1 1] Roatate widget component
  (bind _astop_down_character (Utilities|Casting|CastToTopDownCharacter (Game|GetPlayerCharacter 0))
    (:then
      (Transformation|SetWorldRotation (Variables|Default|GetWidget) (Math|Conversions|RotationFromXVector (Math|Vector|RotateVector (Math|Vector|Normalize (- (Transformation|GetWorldLocation (Variables|/Game/Blueprints/TopDownCharacter.TopDownCharacter_C|GetCamera1 _astop_down_character)) (Transformation|GetWorldLocation (Variables|Default|GetWidget)))) "0, 0, 0")) false false))
    (:CastFailed
      (Development|PrintString "castfail"))))

(event EventBeginPlay
  ;[1 1 1] Roatate widget component
  (if (not (Variables|Default|GetDisableRotateWidget?))
    (Utilities|Time|SetTimerbyEvent (delegate Custom|AlignToCamera) 0.1 true)))

(fn ConstructionScript)