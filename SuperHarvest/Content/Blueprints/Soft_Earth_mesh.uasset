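; Soft-earth terrain actor that generates a flat, subdivided grid at runtime which can be dug one cell at a time.
; BeginPlay builds vertices, colours and triangles with alternating diagonals into a collidable RuntimeMesh section.
; DigMesh snaps a non-negative location to the grid, lowers that cell's vertices, zeroes their vertex alpha and updates the section.
; IsInsideMyBoundary reports whether a location lies within the patch.
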(event Custom|UpdateMesh
  ;[1 1 1] update mesh
  (Class|RuntimeMeshComponent|UpdateMeshSectionBlueprint (Variables|Default|GetRuntimeMesh) 0 (Variables|Default|GetVerticesArray) (Variables|Default|GetTrianglesArray) 0 0 0 0 (Variables|Default|GetColorArray) false false))

(event Custom|DigMesh
  (params (Location :type Vector))
  (bind _verticesarray (Variables|Default|GetVerticesArray))
  (bind _mylocation (Variables|Default|GetMyLocation))
  (bind _subdivisionspergridpoweroftwo (Variables|Default|GetSubdivisionsPerGridPowerOfTwo))
  (bind (_x _y) (Math|Vector|BreakVector _mylocation))
  (bind _returnvalue (+ _subdivisionspergridpoweroftwo 1))
  (Variables|Default|SetInitialDigLocation Location)
  (if (< (.X (Math|Vector|BreakVector (Variables|Default|GetInitialDigLocation))) 0.0)
    (Development|PrintString "Soft earth mesh location is negative. no support for this atm. move to positive location" :!label _label)
    (elif (< (.Y (Math|Vector|BreakVector (Variables|Default|GetInitialDigLocation))) 0.0)
      (goto _label)
      (else
        (Variables|Default|SetDigX (* (.ReturnValue (Math|Float|Division(WholeandRemainder) (.X (Math|Vector|BreakVector (Variables|Default|GetInitialDigLocation))) 1e+02)) 100))
        (Variables|Default|SetDigY (* (.ReturnValue (Math|Float|Division(WholeandRemainder) (.Y (Math|Vector|BreakVector (Variables|Default|GetInitialDigLocation))) 1e+02)) 100))
        (Variables|Default|SetDigX (- (Variables|Default|GetDigX) (Math|Float|Truncate _x)))
        (Variables|Default|SetDigY (- (Variables|Default|GetDigY) (Math|Float|Truncate _y)))
        (Development|PrintString (Utilities|String|ToString(Integer) (Variables|Default|GetDigX)))
        (Development|PrintString (Utilities|String|ToString(Integer) (Variables|Default|GetDigY)))
        (Variables|Default|SetIndexToStartOn (+ (* (/ (Variables|Default|GetDigY) (Variables|Default|GetTrueGridWidth)) (Variables|Default|GetSubdivisionsPerGridPowerOfTwo)) (* (* (/ (Variables|Default|GetDigX) (Variables|Default|GetTrueGridWidth)) (Variables|Default|GetSubdivisionsPerGridPowerOfTwo)) (+ (* (Variables|Default|GetColumnLength) (Variables|Default|GetSubdivisionsPerGridPowerOfTwo)) 1))))
        (Variables|Default|SetVertsToChange (* _returnvalue _returnvalue))
        (Variables|Default|SetVertsPerColumn (+ (Variables|Default|GetSubdivisionsPerGridPowerOfTwo) 1))
        (Variables|Default|SetAddedFirst? false)
        (Utilities|Array|Clear (Variables|Default|GetVerticeIndexToDig))
        (Variables|Default|SetVertCount 0)
        (for _index (range 0 (- (Variables|Default|GetVertsToChange) 1))
          (if (Variables|Default|GetAddedFirst?)
            (if (>= (Variables|Default|GetVertCount) (Variables|Default|GetVertsPerColumn))
              (Variables|Default|SetVertCount 0)
              (Variables|Default|SetVertsToChange (+ (Variables|Default|GetVertsToChange) 1))
              (Variables|Default|SetIndexToStartOn (+ (- (Variables|Default|GetIndexToStartOn) (Variables|Default|GetSubdivisionsPerGridPowerOfTwo)) (* (Variables|Default|GetColumnLength) (Variables|Default|GetSubdivisionsPerGridPowerOfTwo))))
              (else
                (Variables|Default|SetIndexToStartOn (+ (Variables|Default|GetIndexToStartOn) 1))
                (Utilities|Array|Add (Variables|Default|GetVerticeIndexToDig) (Variables|Default|GetIndexToStartOn))
                (Variables|Default|SetVertCount (+ (Variables|Default|GetVertCount) 1))))
            (else
              (Utilities|Array|Add (Variables|Default|GetVerticeIndexToDig) (Variables|Default|GetIndexToStartOn))
              (Variables|Default|SetVertCount (+ (Variables|Default|GetVertCount) 1))
              (Variables|Default|SetAddedFirst? true))))
        (for _array_element (Variables|Default|GetVerticeIndexToDig)
          (Utilities|Array|SetArrayElem _verticesarray _array_element (Math|Vector|MakeVector (.X (Math|Vector|BreakVector (Utilities|Array|Get(acopy) _verticesarray _array_element))) (.Y (Math|Vector|BreakVector (Utilities|Array|Get(acopy) _verticesarray _array_element))) -2e+01))
          (Utilities|Array|SetArrayElem (Variables|Default|GetColorArray) _array_element "(R=0.000000,G=0.000000,B=0.000000,A=0.000000)"))
        (CallFunction|UpdateMesh)))))

(event EventBeginPlay
  (bind _runtimemesh (Variables|Default|GetRuntimeMesh))
  (if (== (Variables|Default|GetSubdivisionsPerGridPowerOfTwo) 0)
    (Development|PrintString "error cant be 0 subdivs")
    (else
      (Variables|Default|SetSubdivisionsWidth (/ (Math|Conversions|ToFloat(Integer) (Variables|Default|GetTrueGridWidth)) (Math|Conversions|ToFloat(Integer) (Variables|Default|GetSubdivisionsPerGridPowerOfTwo))))
      (Variables|Default|SetMyLocation (Transformation|GetWorldLocation (Variables|Default|GetDefaultSceneRoot self)))
      (Variables|Default|SetNumberOfVertices (* (+ (* (Variables|Default|GetColumnLength) (Variables|Default|GetSubdivisionsPerGridPowerOfTwo)) 1) (+ (* (Variables|Default|GetRowLength) (Variables|Default|GetSubdivisionsPerGridPowerOfTwo)) 1)))
      (Variables|Default|SetVertexVectorRef "")
      (Utilities|Array|Clear (Variables|Default|GetColorArray))
      (for _index (range 0 (- (Variables|Default|GetNumberOfVertices) 1))
        (if (Variables|Default|GetAddedFirst?)
          (if (>= (.Y (Math|Vector2D|BreakVector2D (Variables|Default|GetVertexVectorRef))) (Math|Conversions|ToFloat(Integer) (* (Variables|Default|GetTrueGridWidth) (Variables|Default|GetColumnLength))))
            (if (>= (.X (Math|Vector2D|BreakVector2D (Variables|Default|GetVertexVectorRef))) (Math|Conversions|ToFloat(Integer) (* (Variables|Default|GetTrueGridWidth) (Variables|Default|GetRowLength))))
              (Development|PrintString "Too many in forloop")
              (else
                (Variables|Default|SetVertexVectorRef (Math|Vector2D|MakeVector2D (+ (.X (Math|Vector2D|BreakVector2D (Variables|Default|GetVertexVectorRef))) (Variables|Default|GetSubdivisionsWidth)) 0.0))
                (Utilities|Array|Add (Variables|Default|GetVerticesArray) (Math|Vector|MakeVector (.X (Math|Vector2D|BreakVector2D (Variables|Default|GetVertexVectorRef))) (.Y (Math|Vector2D|BreakVector2D (Variables|Default|GetVertexVectorRef))) 0.0))
                (Utilities|Array|Add (Variables|Default|GetColorArray) "(R=0.000000,G=0.000000,B=0.000000,A=1.000000)")))
            (else
              (Variables|Default|SetVertexVectorRef (Math|Vector2D|MakeVector2D (.X (Math|Vector2D|BreakVector2D (Variables|Default|GetVertexVectorRef))) (+ (.Y (Math|Vector2D|BreakVector2D (Variables|Default|GetVertexVectorRef))) (Variables|Default|GetSubdivisionsWidth))))
              (Utilities|Array|Add (Variables|Default|GetVerticesArray) (Math|Vector|MakeVector (.X (Math|Vector2D|BreakVector2D (Variables|Default|GetVertexVectorRef))) (.Y (Math|Vector2D|BreakVector2D (Variables|Default|GetVertexVectorRef))) 0.0))
              (Utilities|Array|Add (Variables|Default|GetColorArray) "(R=0.000000,G=0.000000,B=0.000000,A=1.000000)")))
          (else
            (Utilities|Array|Add (Variables|Default|GetVerticesArray) (Math|Vector|MakeVector (.X (Math|Vector2D|BreakVector2D (Variables|Default|GetVertexVectorRef))) (.Y (Math|Vector2D|BreakVector2D (Variables|Default|GetVertexVectorRef))) 0.0))
            (Variables|Default|SetAddedFirst? true)
            (Utilities|Array|Add (Variables|Default|GetColorArray) "(R=0.000000,G=0.000000,B=0.000000,A=1.000000)"))))
      (Variables|Default|SetTranglesToBuild (* (+ (* (Variables|Default|GetColumnLength) (Variables|Default|GetSubdivisionsPerGridPowerOfTwo)) 1) (* (Variables|Default|GetRowLength) (Variables|Default|GetSubdivisionsPerGridPowerOfTwo))))
      (Variables|Default|SetFlipTriangleMax (/ (+ (Variables|Default|GetSubdivisionsPerGridPowerOfTwo) 2) 2))
      (Variables|Default|SetIndexToReverseTriangleDirection (* (* (Variables|Default|GetColumnLength) (Variables|Default|GetSubdivisionsPerGridPowerOfTwo)) (+ (/ (Variables|Default|GetSubdivisionsPerGridPowerOfTwo) 2) 1)))
      (for _index_2 (range 0 (- (Variables|Default|GetTranglesToBuild) 1))
        (Variables|Default|SetIndex _index_2)
        (if (== (Variables|Default|GetIndex) (Variables|Default|GetIndexToReverseTriangleDirection))
          (CallFunction|FlipFlopBool)
          (Variables|Default|SetIndexToReverseTriangleDirection (+ (Variables|Default|GetIndexToReverseTriangleDirection) (Variables|Default|GetIndexToReverseTriangleDirection))))
        (Variables|Default|SetSkipCount (+ (Variables|Default|GetSkipCount) 1))
        (if (== (Variables|Default|GetSkipCount) (+ (* (Variables|Default|GetColumnLength) (Variables|Default|GetSubdivisionsPerGridPowerOfTwo)) 1))
          (Variables|Default|SetSkipCount 0)
          (Variables|Default|SetTranglesToBuild (+ (Variables|Default|GetTranglesToBuild) 1))
          (else
            (Variables|Default|SetFlipTriangleCount (+ (Variables|Default|GetFlipTriangleCount) 1))
            (if (<= (Variables|Default|GetFlipTriangleCount) (Variables|Default|GetFlipTriangleMax))
              (if (Variables|Default|GetDirectionFlipped?) :!label _label
                (CallFunction|RegularDirectionTriangles)
                (else
                  (CallFunction|InverseDirectionTriangles)))
              (elif (<= (Variables|Default|GetFlipTriangleCount) (* (Variables|Default|GetFlipTriangleMax) 2))
                (if (Variables|Default|GetDirectionFlipped?)
                  (CallFunction|InverseDirectionTriangles)
                  (else
                    (CallFunction|RegularDirectionTriangles)))
                (else
                  (Variables|Default|SetFlipTriangleCount 0)
                  (Variables|Default|SetFlipTriangleCount (+ (Variables|Default|GetFlipTriangleCount) 1))
                  (goto _label)))))))
      (Class|RuntimeMeshComponent|CreateMeshSectionBlueprint _runtimemesh 0 (Variables|Default|GetVerticesArray) (Variables|Default|GetTrianglesArray) 0 0 0 0 (Variables|Default|GetColorArray) true false false "Average")
      (Rendering|Material|SetMaterial _runtimemesh 0 "/Game/Assets/Materials/Soft_Earth_Master_Inst.Soft_Earth_Master_Inst"))))

(fn ConstructionScript)

(fn IsInsideMyBoundary?
  (params (DigLocation :type Vector))
  (bind (_x _y) (Math|Vector|BreakVector DigLocation))
  (bind _mylocation (Variables|Default|GetMyLocation))
  (bind _mylocation_2 (Variables|Default|GetMyLocation))
  (bind _y_2 (Math|Vector|BreakVector _mylocation))
  (bind _x_2 (Math|Vector|BreakVector _mylocation_2))
  (if (Math|Float|InRange(Float) _x _x_2 (+ _x_2 (Math|Conversions|ToFloat(Integer) (* (Variables|Default|GetColumnLength) (Variables|Default|GetTrueGridWidth)))))
    (if (Math|Float|InRange(Float) _y _y_2 (+ _y_2 (Math|Conversions|ToFloat(Integer) (* (Variables|Default|GetColumnLength) (Variables|Default|GetTrueGridWidth)))))
      (LocalVariables|SetIsInside? true)
      (else
        (LocalVariables|SetIsInside? false :!label _label)))
    (else
      (goto _label)))
  (return (LocalVariables|GetIsInside?)))

(fn RegularDirectionTriangles
  (bind _index (Variables|Default|GetIndex))
  ;[1 1 1] regular direction triangles
  (Utilities|Array|Add (Variables|Default|GetTrianglesArray) _index)
  (Utilities|Array|Add (Variables|Default|GetTrianglesArray) (+ _index 1))
  (Utilities|Array|Add (Variables|Default|GetTrianglesArray) (+ (+ (+ (* (Variables|Default|GetColumnLength) (Variables|Default|GetSubdivisionsPerGridPowerOfTwo)) 1) _index) 1))
  (Utilities|Array|Add (Variables|Default|GetTrianglesArray) _index)
  (Utilities|Array|Add (Variables|Default|GetTrianglesArray) (+ (+ (+ (* (Variables|Default|GetColumnLength) (Variables|Default|GetSubdivisionsPerGridPowerOfTwo)) 1) _index) 1))
  (Utilities|Array|Add (Variables|Default|GetTrianglesArray) (+ (+ (* (Variables|Default|GetColumnLength) (Variables|Default|GetSubdivisionsPerGridPowerOfTwo)) 1) _index)))

(fn InverseDirectionTriangles
  (bind _index (Variables|Default|GetIndex))
  ;[1 1 1] inversed direction triangles
  (Utilities|Array|Add (Variables|Default|GetTrianglesArray) (+ _index 1))
  (Utilities|Array|Add (Variables|Default|GetTrianglesArray) (+ (+ (+ (* (Variables|Default|GetColumnLength) (Variables|Default|GetSubdivisionsPerGridPowerOfTwo)) 1) _index) 1))
  (Utilities|Array|Add (Variables|Default|GetTrianglesArray) (+ (+ (* (Variables|Default|GetColumnLength) (Variables|Default|GetSubdivisionsPerGridPowerOfTwo)) 1) _index))
  (Utilities|Array|Add (Variables|Default|GetTrianglesArray) (+ _index 1))
  (Utilities|Array|Add (Variables|Default|GetTrianglesArray) (+ (+ (* (Variables|Default|GetColumnLength) (Variables|Default|GetSubdivisionsPerGridPowerOfTwo)) 1) _index))
  (Utilities|Array|Add (Variables|Default|GetTrianglesArray) _index))

(fn FlipFlopBool
  (if (Variables|Default|GetDirectionFlipped?)
    (Variables|Default|SetDirectionFlipped? false)
    (else
      (Variables|Default|SetDirectionFlipped? true)))
  (return))