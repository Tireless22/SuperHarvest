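; Talking NPC for the top-down game that wears random showcase gear, slaved to its body mesh via master pose.
; A talk-radius overlap eases clamped head and chest look-at rotations toward the player through timelines and a tick-fed gate.
; StartDialogue cycles through lines, typing each with blip sounds, while a looping timer ends dialogue when the player walks away.
; Tick polls the UI_Clock widget to scale a hand-held torch in at night and out by day.
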(event OnComponentEndOverlap(TalkRadius)
  (params (OverlappedComponent :type Primitive%20Component%20Object%20Reference) (OtherActor :type Actor%20Object%20Reference) (OtherComp :type Primitive%20Component%20Object%20Reference) (OtherBodyIndex :type Integer))
  ;[1 1 1] on end overlap with topdownchar set in range to false and en lookat
  (if (Utilities|Enum|Equal(Enum) (Utilities|GetDisplayName OtherActor) "TopDownCharacter")
    (Variables|Default|SetIsInRange? false)
    (Utilities|FlowControl|Delay 1.0)
    (if (not (Variables|Default|GetIsInRange?))
      (CallFunction|EndLookat))))

(event OnComponentBeginOverlap(TalkRadius)
  (params (OverlappedComponent :type Primitive%20Component%20Object%20Reference) (OtherActor :type Actor%20Object%20Reference) (OtherComp :type Primitive%20Component%20Object%20Reference) (OtherBodyIndex :type Integer) (bFromSweep :type Boolean) (SweepResult :type Hit%20Result%20Structure%20%28by%20ref%29))
  ;[1 1 1] on overlap with topdown char set is in range to true, start lookat
  (if (Utilities|Enum|Equal(Enum) (Utilities|GetDisplayName OtherActor) "TopDownCharacter")
    (Variables|LookAt|SetLookAtActor OtherActor)
    (Variables|Default|SetIsInRange? true)
    (CallFunction|LookatStart)))

(event Custom|StartDialogue
  ;[1 1 1] Start timer, create dialogue widget, start dialogue
  (Variables|Default|SetIsEnded? false)
  (bind _returnvalue (Utilities|Time|SetTimerbyEvent (delegate Custom|CheckDistanceToPawn) 0.5 true))
  (bind _returnvalue_2 (UserInterface|CreateWidget "/Game/UI/UI_NPC_Dialogue.UI_NPC_Dialogue_C" (Game|GetPlayerController 0)))
  (Variables|Default|SetUI_NPC_DIalogue_ref _returnvalue_2)
  (UserInterface|Viewport|AddtoViewport _returnvalue_2 0)
  (if (> (+ (Variables|Default|GetCurrentDialogueIndex) 1) (- (Utilities|Array|Length (Variables|Default|GetDialogues)) 1))
    (Variables|Default|SetCurrentDialogueIndex 0)
    (else
      (Variables|Default|SetCurrentDialogueIndex (+ (Variables|Default|GetCurrentDialogueIndex) 1))))
  (Utilities|ScrollTextLetterbyLetter (Variables|/Game/UI/UI_NPC_Dialogue.UI_NPC_Dialogue_C|GetDialogueText _returnvalue_2) (Utilities|Array|Get(acopy) (Variables|Default|GetDialogues) (Variables|Default|GetCurrentDialogueIndex)) 0.04))

(event Custom|EndDialogue
  ;[1 1 1] End dialogue
  (Variables|Default|SetIsEnded? true)
  (Variables|Default|SetArrayIndexValue 0)
  (Variables|Default|SetAppendedTextString "")
  (Utilities|Time|ClearandInvalidateTimerbyHandle (stale Custom|StartDialogue _returnvalue))
  (bind _astop_down_character (Utilities|Casting|CastToTopDownCharacter (Game|GetPlayerCharacter 0))
    (:then
      (Variables|/Game/Blueprints/TopDownCharacter.TopDownCharacter_C|SetIsInDialogue? _astop_down_character false)
      (Widget|RemovefromParent (Variables|Default|GetUI_NPC_DIalogue_ref)))
    (:CastFailed
      (Development|PrintString "cast fail"))))

(event Custom|EndLookAt
  ;[1 1 1] Lerp Into Look At
  (Variables|LookAt|SetLookAtActor 0)
  (Variables|LookAt|SetLookAt_tmp (Variables|LookAt|GetLookAt))
  (Variables|LookAt|SetLookAtChest_tmp (Variables|LookAt|GetLookAtChest))
  (bind _newtrack_0 (Timeline|End PlayFromStart)
    (:Update
      (Variables|LookAt|SetLookAtChest (Math|Rotator|Lerp(Rotator) (Variables|LookAt|GetLookAtChest_tmp) "0, 0, 0" _newtrack_0))
      (Variables|LookAt|SetLookAt (Math|Rotator|Lerp(Rotator) (Variables|LookAt|GetLookAt_tmp) "0, 0, 0" _newtrack_0)))
    (:Finished
      ;[1 1 1] LookAt (bit buggy)
      (Utilities|FlowControl|Gate true) ; enters at Close
    )))

(event Custom|LookAtStart
  ;[1 1 1] Lerp Into Look At
  (Variables|LookAt|SetLookAtChest_tmp (CallFunction|GetChestLookat "Spine3"))
  (Variables|LookAt|SetLookAt_tmp (CallFunction|GetHeadLookat))
  (bind _newtrack_0 (Timeline|start PlayFromStart)
    (:Update
      (Variables|LookAt|SetLookAtChest (Math|Rotator|Lerp(Rotator) "0, 0, 0" (Variables|LookAt|GetLookAtChest_tmp) _newtrack_0))
      (Variables|LookAt|SetLookAt (Math|Rotator|Lerp(Rotator) "0, 0, 0" (Variables|LookAt|GetLookAt_tmp) _newtrack_0)))
    (:Finished
      ;[1 1 1] LookAt (bit buggy)
      (Utilities|FlowControl|Gate true) ; enters at Open
    )))

(event Custom|CheckDistanceToPawn
  ;[1 1 1] CheckDistance to topdownchar, if too far end dialogue
  (bind _astop_down_character (Utilities|Casting|CastToTopDownCharacter (Game|GetPlayerCharacter 0))
    (:then
      (if (> (Math|Vector|VectorLength (- (Transformation|GetWorldLocation (Variables|/Script/Engine.Character|GetMesh _astop_down_character)) (Transformation|GetWorldLocation (Variables|Default|GetNPC)))) 2e+02)
        (CallFunction|EndDialogue)))
    (:CastFailed
      (Development|PrintString "fail cast"))))

(event EventBeginPlay
  (bind _chest_meshes (Utilities|Struct|MakeChest_Meshes "/Game/Assets/Equipment/Chest/Jacket_01/Jacket_01.Jacket_01" "/Game/Assets/Equipment/Chest/Admirals_Chest/Admirals_Chest.Admirals_Chest"))
  (bind _legs_meshes (Utilities|Struct|Makelegs_Meshes "/Game/Assets/Equipment/Legs/Admirals_Pants/Admirals_Pants.Admirals_Pants" "/Game/Assets/Equipment/Legs/Shorts_Striped_01/Shorts_Striped_01.Shorts_Striped_01"))
  (bind _feet_meshes (Utilities|Struct|MakeFeet_Meshes "/Game/Assets/Equipment/Feet/Boots_01/Boots_01.Boots_01" "/Game/Assets/Equipment/Feet/Admirals_Boots/Admirals_Boots.Admirals_Boots"))
  (bind (_chest_01 _chest_02) (Utilities|Struct|BreakChest_Meshes _chest_meshes))
  (bind (_legs_01 _legs_02) (Utilities|Struct|Breaklegs_Meshes _legs_meshes))
  (bind (_feet_01 _feet_02) (Utilities|Struct|BreakFeet_Meshes _feet_meshes))
  (bind _array (Utilities|Array|MakeArray _feet_01 _feet_02))
  (bind _array_2 (Utilities|Array|MakeArray _chest_01 _chest_02))
  (bind _array_3 (Utilities|Array|MakeArray _legs_01 _legs_02))
  ;[1 1 1] Event Begin Play
  ;[1 1 1] Set Random Gear (Showcase)
  (Variables|Gear|SetSetChestMesh (Utilities|Array|Get(acopy) _array_2 (Math|Random|RandomIntegerinRange 0 (- (Utilities|Array|Length _array_2) 1))))
  (Variables|Gear|SetSetLegMesh (Utilities|Array|Get(acopy) _array_3 (Math|Random|RandomIntegerinRange 0 (- (Utilities|Array|Length _array_3) 1))))
  (Variables|Gear|SetSetBootMesh (Utilities|Array|Get(acopy) _array (Math|Random|RandomIntegerinRange 0 (- (Utilities|Array|Length _array) 1))))
  (CallFunction|SetGear (Variables|Default|GetChest) (Variables|Gear|GetSetChestMesh))
  (CallFunction|SetGear (Variables|Default|GetLegs) (Variables|Gear|GetSetLegMesh))
  (CallFunction|SetGear (Variables|Default|GetBoots) (Variables|Gear|GetSetBootMesh)))

(event EventTick
  (params (DeltaSeconds :type Float%20%28single-precision%29))
  ;[1 1 1] Event Tick (Better way to do it?)
  (Utilities|FlowControl|Sequence
    (:then_0
      ;[1 1 1] LookAt (bit buggy)
      (if (Variables|Default|GetIsInRange?)
        (Utilities|FlowControl|Gate true
          (:Exit
            (Variables|LookAt|SetLookAtChest (CallFunction|GetChestLookat "Spine3"))
            (Variables|LookAt|SetLookAt (CallFunction|GetHeadLookat))))))
    (:then_1
      ;[1 1 1] Takes out torch during night time
      (bind _foundwidgets (Widget|GetAllWidgetsOfClass "/Game/UI/UI_Clock.UI_Clock_C" true))
      (if (or (< (Variables|/Game/UI/UI_Clock.UI_Clock_C|GetCurrentHour (Utilities|Array|Get(acopy) _foundwidgets)) 7.0) (> (Variables|/Game/UI/UI_Clock.UI_Clock_C|GetCurrentHour (Utilities|Array|Get(acopy) _foundwidgets)) 19.0))
        (Variables|Default|SetIsNight true)
        (Utilities|FlowControl|DoOnce false :!label _label
          (:Completed
            (bind _returnvalue (AddComponent|AddChildActorComponent true))
            (Transformation|AttachComponentToComponent _returnvalue (Variables|Default|GetNPC) "RightHandSocket" "SnapToTarget" "SnapToTarget" "KeepRelative" true)
            (bind _newtrack_0 (Timeline|Timeline_1 PlayFromStart)
              (:Update
                (Transformation|SetWorldScale3D _returnvalue (Math|Vector|Lerp(Vector) "0.000000,0.000000,0.000000" "1.000000,1.000000,1.000000" _newtrack_0)))
              (:Finished
                (goto _label_2 Reset)))))
        (else
          (Variables|Default|SetIsNight false)
          (Utilities|FlowControl|DoOnce false :!label _label_2
            (:Completed
              (bind _newtrack_0_2 (Timeline|Timeline_0 Play)
                (:Update
                  (Transformation|SetWorldScale3D _returnvalue (Math|Vector|Lerp(Vector) "1.000000,1.000000,1.000000" "0, 0, 0" _newtrack_0_2)))
                (:Finished
                  (Components|DestroyComponent _returnvalue)
                  (goto _label Reset))))))))))

(fn ConstructionScript)

(fn SetGear
  (params (GearType :type Skeletal%20Mesh%20Component%20Object%20Reference) (GearMesh :type Skeletal%20Mesh%20Object%20Reference))
  (Class|SkinnedMeshComponent|SetSkeletalMesh GearType GearMesh true)
  (Class|SkinnedMeshComponent|SetMasterPoseComponent GearType (Variables|Default|GetNPC)))

(fn GetHeadLookat
  (bind _npc (Variables|Default|GetNPC))
  (bind _lookatactor (Variables|LookAt|GetLookAtActor))
  (bind _returnvalue (Transformation|GetActorLocation _lookatactor))
  (bind _returnvalue_2 (Transformation|GetSocketLocation _npc "HeadSocket"))
  (bind _returnvalue_3 (+ _returnvalue "0, 0,15.000000"))
  (bind _returnvalue_4 (Math|Rotator|FindLookatRotation _returnvalue_3 _returnvalue_2))
  (bind _yaw (Math|Rotator|BreakRotator _returnvalue_4))
  (bind _returnvalue_5 (Math|Float|Clamp(Float) _yaw -9e+01 9e+01))
  (bind _returnvalue_6 (Math|Rotator|MakeRotator 0.0 0.0 _returnvalue_5))
  (bind (_roll _pitch _yaw_2) (Math|Rotator|BreakRotator _returnvalue_6))
  (return (Math|Rotator|MakeRotator _roll _pitch (- (- _yaw_2 (.Yaw (Math|Rotator|BreakRotator (* (CallFunction|GetChestLookat "Spine3") 0.4)))) (.Yaw (Math|Rotator|BreakRotator (* (CallFunction|GetChestLookat "Spine2") 0.2)))))))

(fn GetChestLookat
  (params (SocketName :type Name))
  (return (Math|Rotator|MakeRotator 0.0 0.0 (Math|Float|Clamp(Float) (.Yaw (Math|Rotator|BreakRotator (Math|Rotator|FindLookatRotation (+ (Transformation|GetActorLocation (Variables|LookAt|GetLookAtActor)) "0, 0,15.000000") (Transformation|GetSocketLocation (Variables|Default|GetNPC) SocketName)))) -4e+01 4e+01))))