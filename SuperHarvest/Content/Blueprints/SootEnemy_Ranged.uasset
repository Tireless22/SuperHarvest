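; Ranged soot enemy AI character that spawns a crossbow in its hand and fires at players it sees.
; A looping server timer picks a TopDownCharacter via sight perception, then drives aiming, range-based movement and firing.
; The same timer fades the health bar widget by local player proximity.
; Damage flashes a material red and updates health; death multicasts ragdoll, rolls data-table loot and destroys the actor after a delay.
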(event Custom|MainEvents
  (bind _returnvalue (Game|GetPlayerController 0))
  (bind _self self)
  (bind _returnvalue_2 (Pawn|GetControlledPawn _returnvalue))
  ;[1 1 1] AI
  (Networking|SwitchHasAuthority
    (:Authority
      (Utilities|FlowControl|Sequence
        (:then_1
          ;[1 1 1] Select Target
          (if (== (Variables|Default|GetTopDownCharacterReference) 0)
            (for _array_element (Class|AIPerceptionComponent|GetCurrentlyPerceivedActors (Variables|Default|GetAIPerception) "/Script/AIModule.AISense_Sight")
              (if (== (Utilities|GetClass _array_element) "/Game/Blueprints/TopDownCharacter.TopDownCharacter_C")
                (Variables|Default|SetCurrentDistanceTo (Transformation|GetDistanceTo _array_element self))
                (if (<= (Transformation|GetDistanceTo _array_element self) (Variables|Default|GetCurrentDistanceTo))
                  (bind _astop_down_character (Utilities|Casting|CastToTopDownCharacter _array_element))
                  (Variables|Default|SetTopDownCharacterReference _astop_down_character))))
            (else
              (for _array_element_2 (Class|AIPerceptionComponent|GetCurrentlyPerceivedActors (Variables|Default|GetAIPerception) "/Script/AIModule.AISense_Sight")
                (if (== _array_element_2 (Variables|Default|GetTopDownCharacterReference))
                  (CallFunction|MultiCastArrowtoThreat)
                  (else
                    (Variables|Default|SetTopDownCharacterReference 0)))))))
        (:then_2
          ;[1 1 1] MoveToActor
          (Utilities|IsValid (Variables|Default|GetTopDownCharacterReference)
            (:Is%20Valid
              (if (not (<= (Transformation|GetDistanceTo (Variables|Default|GetTopDownCharacterReference)) (Variables|Default|GetVisionRange)))
                (if (<= (Transformation|GetDistanceTo (Variables|Default|GetTopDownCharacterReference)) (Variables|Default|GetAttackRange))
                  (Components|Movement|StopMovementImmediately (Variables|/Script/Engine.Character|GetCharacterMovement _self))
                  (Development|PrintString "AI: STOP for aim")
                  (else
                    (AI|Navigation|SimpleMovetoActor (AI|GetAIController _self) (Variables|Default|GetTopDownCharacterReference))))))))
        (:then_3
          ;[1 1 1] Attack when within 100units. Wants to be moved to BlackBoard
          (Utilities|IsValid (Variables|Default|GetTopDownCharacterReference)
            (:Is%20Valid
              (if (<= (Transformation|GetDistanceTo (Variables|Default|GetTopDownCharacterReference)) (Variables|Default|GetAttackRange)) :!label _label
                (Default|Fire (Variables|Default|GetWeapon))
                (Variables|Default|SetAttack true)
                (Utilities|FlowControl|Delay 1.0)
                (Variables|Default|SetAttack false)
                (goto _label)
                (else
                  (Variables|Default|SetAttack false))))))
        (:then_6
          ;[1 1 1] UI Fade (Doesn't need to be networked, right?)
          (Utilities|IsValid _returnvalue_2 :!label _label_2
            (:Is%20Valid
              (if (<= (Transformation|GetDistanceTo _returnvalue_2) 6e+02)
                (if (not (Variables|Default|GetCalledFadeOut?))
                  (Variables|Default|SetCalledFadeOut? true)
                  (CallFunction|FadeUI true))
                (elif (Variables|Default|GetCalledFadeOut?)
                  (Variables|Default|SetCalledFadeOut? false)
                  (CallFunction|FadeUI false))))))))
    (:Remote
      (goto _label_2))))

(event Custom|MultiCast_ArrowToThreat
  ;[1 1 1] Select Target
  (Transformation|SetWorldRotation (Variables|Default|GetTHREAT) (Math|Rotator|FindLookatRotation (Transformation|GetWorldLocation (Variables|Character|GetMesh)) (Transformation|GetWorldLocation (Variables|/Script/Engine.Character|GetMesh (Variables|Default|GetTopDownCharacterReference)))) false false))

(event Custom|MultiCast_EventBegin
  ;[1 1 1] BeginPlay
  (CallFunction|UpdateUIHealth))

(event Custom|Soot%20Enemy%20Damage%20Visibility
  (bind _mesh (Variables|Character|GetMesh))
  ;[1 1 1] Damage Shader Toggle
  (Rendering|Material|SetMaterial _mesh 4 "/Game/Assets/Materials/Emissive_Red.Emissive_Red")
  (Utilities|FlowControl|Delay 0.15)
  (Rendering|Material|SetMaterial _mesh 4 (Variables|Default|GetSootBodyColor)))

(event Custom|MultiCast_HitEffect
  ;[1 1 1] TakeDamage
  ;;[1 1 1] Update HP Text
  (Effects|SpawnEmitteratLocation "/Game/VFX/leaf_fall_small.leaf_fall_small" (Transformation|GetActorLocation)) ; HitReaction Effect (Blood?)
  (CallFunction|UpdateUIHealth))

(event Custom|MultiCast_Death
  (bind _mesh (Variables|Character|GetMesh))
  ;[1 1 1] TakeDamage
  ;;[1 1 1] disable event loop
  (Utilities|Time|ClearandInvalidateTimerbyHandle (Variables|Default|GetMainTimerHandle))
  (Effects|SpawnEmitteratLocation "/Game/VFX/grass_straw_cloud_01.grass_straw_cloud_01" (Transformation|GetActorLocation))
  ;;[1 1 1] Death
  ;;;[1 1 1] Disable More! No Anim, No Ai
  (Pawn|Components|CharacterMovement|DisableMovement (Variables|Character|GetCharacterMovement))
  (Physics|SetSimulatePhysics _mesh true)
  (Collision|SetCollisionResponsetoChannel _mesh "ECC_Pawn" "ECR_Ignore")
  (Utilities|FlowControl|Sequence
    (:then_2
      (Components|Animation|SetAnimationMode (Variables|Character|GetMesh) "AnimationSingleNode"))
    (:then_3
      (Collision|SetCollisionEnabled (Variables|Collision|GetCapsuleComponent) "NoCollision"))
    (:then_4
      (CallFunction|SpawnLoot))
    (:then_5
      (Rendering|SetVisibility (Variables|Default|GetWidget) false false))
    (:then_6
      (Utilities|FlowControl|Delay 8.0)
      (Actor|DestroyActor))))

(event EventBeginPlay
  (bind _self self)
  ;[1 1 1] BeginPlay
  (Utilities|FlowControl|Delay 1.0) ; Wait til all players has loaded here
  (bind _returnvalue (Utilities|Time|SetTimerbyEvent (delegate Custom|MainEvents) 0.5 true))
  (Variables|Default|SetMainTimerHandle _returnvalue)
  (Networking|SwitchHasAuthority
    (:Authority
      (Variables|Default|SetStartHealth (Variables|Default|GetHealth))
      (Variables|Default|SetStartRunSpeed (Variables|/Script/Engine.CharacterMovementComponent|GetMaxWalkSpeed (Variables|Character|GetCharacterMovement)))
      (Variables|Default|SetStartWalkSpeed 2e+02)
      (Variables|Default|SetSootBodyColor (Rendering|Material|GetMaterial (Variables|Character|GetMesh) 4))
      (bind _returnvalue_2 (Game|SpawnActorfromClass "/Game/Interactibles/Weapons/EnemyWeapon/Soot_Crossbow.Soot_Crossbow_C" (Transformation|GetActorTransform) "Undefined" _self false true _self))
      (bind _output_get (Variables|Default|SetWeapon _returnvalue_2))
      (Transformation|AttachComponentToComponent _output_get (Variables|Character|GetMesh) "LeftHand_ItemJoint" "SnapToTarget" "SnapToTarget" "SnapToTarget" false)
      (Utilities|FlowControl|Delay 0.5)
      (CallFunction|MultiCastEventBegin))))

(event Game|Damage|EventAnyDamage
  (params (Damage :type Float%20%28single-precision%29) (DamageType :type Damage%20Type%20Object%20Reference) (InstigatedBy :type Controller%20Object%20Reference) (DamageCauser :type Actor%20Object%20Reference))
  ;[1 1 1] TakeDamage
  (Variables|Default|SetHealth (- (Variables|Default|GetHealth) Damage))
  (CallFunction|SootEnemyDamageVisibility)
  (if (<= (Variables|Default|GetHealth) 0.0)
    (CallFunction|MultiCastDeath)
    (else
      ;;[1 1 1] Update HP Text
      (CallFunction|MultiCastHitEffect))))

(fn ConstructionScript)

(fn SpawnLoot
  (Development|PrintString "Rolling for loot!")
  (bind _outrownames (DataTable|GetDataTableRowNames "/Game/Interactibles/Soot_LootList.Soot_LootList"))
  (for _array_element _outrownames
    (bind _returnvalue (Utilities|GetDataTableRow "/Game/Interactibles/Soot_LootList.Soot_LootList" _array_element)
      (:then
        (LocalVariables|SetDropChance (.DropChance (Utilities|Struct|BreakLootList _returnvalue)))
        (LocalVariables|SetIDName (.ID (Utilities|Struct|BreakLootList _returnvalue)))
        (LocalVariables|SetMaxAmount (.MaxAmount (Utilities|Struct|BreakLootList _returnvalue)))
        (LocalVariables|SetClassRef (.ActorClass (Utilities|Struct|BreakLootList _returnvalue)))
        (LocalVariables|SetMinAmount (.MinAmount (Utilities|Struct|BreakLootList _returnvalue)))
        (if (Math|Float|InRange(Float) (Math|Random|RandomFloatinRange 0.0 1.0) 0.0 (LocalVariables|GetDropChance))
          (for _index (range (LocalVariables|GetMinAmount) (LocalVariables|GetMaxAmount))
            (bind _asbp_base_item (Utilities|Casting|CastToBP_BaseItemClass (LocalVariables|GetClassRef)))
            (Game|SpawnActorfromClass _asbp_base_item (Transformation|GetWorldTransform (Variables|Character|GetMesh)) "Undefined" 0 true false 0))
          (else
            (Development|PrintString "rolled for no loot" true true "(R=0.347548,G=0.000000,B=1.000000,A=1.000000)"))))
      (:RowNotFound
        (Development|PrintString "Error did not find row")))))

(fn UpdateUIHealth
  (bind _asui_health_bar (Utilities|Casting|CastToUI_HealthBar (UserInterface|GetUserWidgetObject (Variables|Default|GetWidget)))
    (:then
      (Variables|/Game/UI/UI_HealthBar.UI_HealthBar_C|SetHealthPercent _asui_health_bar (/ (Variables|Default|GetHealth) (Variables|Default|GetStartHealth))))
    (:CastFailed
      (Development|PrintString "castfail"))))

(fn FadeUI
  (params (FadeOut? :type Boolean))
  (LocalVariables|SetRef FadeOut?)
  (bind _asui_health_bar (Utilities|Casting|CastToUI_HealthBar (UserInterface|GetUserWidgetObject (Variables|Default|GetWidget)))
    (:then
      (Default|SetStartFade _asui_health_bar (LocalVariables|GetRef)))
    (:CastFailed
      (Development|PrintString "castfail"))))