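; Earth mesh Blueprint that shows a piece of ground with randomized scattered earth and a burst of earth chips on spawn.
; BeginPlay spawns the chip emitter just above the secondary mesh, then randomizes that mesh's yaw and sinks it slightly.
; SetMyMesh takes a type from 1 to 4 to give the main mesh a random variant from that type's array.
; Its first call also assigns a fixed earth-pieces mesh to the secondary component.
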(event Custom|SetMyMesh
  (params (MeshTypeInfo :type Integer))
  (Variables|Default|SetMyInfoType MeshTypeInfo)
  (Utilities|FlowControl|Sequence
    (:then_0
      (switch int (Variables|Default|GetMyInfoType)
        (:1
          (CallFunction|SetMesh (Variables|Default|GetMeshType1)))
        (:2
          (CallFunction|SetMesh (Variables|Default|GetMeshType2)))
        (:3
          (CallFunction|SetMesh (Variables|Default|GetMeshType3)))
        (:4
          (CallFunction|SetMesh (Variables|Default|GetMeshType4)))))
    (:then_1
      (if (not (Variables|Default|GetEarthMeshSet?))
        (Variables|Default|SetEarthMeshSet? true)
        (Components|StaticMesh|SetStaticMesh (Variables|Default|GetStaticMesh_02) "/Game/Assets/Meshes/PlowedEarth/earth_pieces_04.earth_pieces_04")))))

(event EventBeginPlay
  (bind _staticmesh_02 (Variables|Default|GetStaticMesh_02))
  (bind _staticmesh_02_2 (Variables|Default|GetStaticMesh_02))
  (bind _returnvalue (Transformation|GetWorldLocation _staticmesh_02_2))
  (bind _returnvalue_2 (Transformation|GetWorldLocation _staticmesh_02))
  (bind (_x _y _z) (Math|Vector|BreakVector _returnvalue))
  (bind (_x_2 _y_2) (Math|Vector|BreakVector _returnvalue_2))
  (Variables|Default|SetEarthIndex (Math|Random|RandomIntegerinRange 0 (- (Utilities|Array|Length (Variables|Default|GetScatteredEarth)) 1)))
  (Effects|SpawnEmitteratLocation "/Game/Assets/VFX/earth_chips_01.earth_chips_01" (Math|Vector|MakeVector _x _y (+ _z 4e+01)))
  (Transformation|SetWorldRotation _staticmesh_02 (Math|Rotator|MakeRotator 0.0 0.0 (Math|Random|RandomFloatinRange 0.0 3.6e+02)) false false)
  (Transformation|SetWorldLocation _staticmesh_02 (Math|Vector|MakeVector _x_2 _y_2 (Math|Random|RandomFloatinRange -2.0 0.0)) false false))

(fn ConstructionScript)

(fn SetMesh
  (params (Array :type Array%20of%20Static%20Mesh%20Object%20References))
  (Components|StaticMesh|SetStaticMesh (Variables|Default|GetStaticMesh) (Utilities|Array|Get(acopy) Array (Math|Random|RandomIntegerinRange 0 (- (Utilities|Array|Length Array) 1)))))