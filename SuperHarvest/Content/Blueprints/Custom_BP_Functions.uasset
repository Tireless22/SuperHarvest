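; Blueprint function library of shared helpers for random chance rolls, player character access and item data lookups.
; Percentage rolls a random integer from 0 to 100 and tests whether it falls within the given chance.
; CastToTopDownChar returns player 0 as a TopDownCharacter, printing a message if the cast fails.
; Three getters fetch weapon, item and armor rows by ID from their data tables, printing an on-screen error when a row is missing.
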(fn Percentage
  (params (Percentage :type Integer))
  (return (Math|Float|InRange(Float) (Math|Conversions|ToFloat(Integer) (Math|Random|RandomIntegerinRange 0 100)) 0.0 (Math|Conversions|ToFloat(Integer) Percentage))))

(fn CasttoTopDownChar
  (bind _astop_down_character (Utilities|Casting|CastToTopDownCharacter (Game|GetPlayerCharacter 0))
    (:then
      (return _astop_down_character))
    (:CastFailed
      (Development|PrintString 0 "Cast to topdown char failed"))))

(fn GetWeaponInfo
  (params (ID :type Name))
  (bind _returnvalue (Utilities|GetDataTableRow "/Game/Interactibles/WeaponInfo.WeaponInfo" ID)
    (:then
      _)
    (:RowNotFound
      (Development|PrintString 0 "ERROR! Could not find Weapon Info!" true true "(R=0.615187,G=0.000000,B=1.000000,A=1.000000)" 4.0)))
  (return _returnvalue))

(fn GetItemInfo
  (params (ID :type Name))
  (bind _returnvalue (Utilities|GetDataTableRow "/Game/Interactibles/ItemInfo.ItemInfo" ID)
    (:then
      _)
    (:RowNotFound
      (Development|PrintString 0 "ERROR! Could not find Item Info!" true true "(R=0.615187,G=0.000000,B=1.000000,A=1.000000)" 4.0)))
  (return _returnvalue))

(fn GetIArmorInfo
  (params (ID :type Name))
  (bind _returnvalue (Utilities|GetDataTableRow "/Game/Interactibles/ArmorInfo.ArmorInfo" ID)
    (:then
      _)
    (:RowNotFound
      (Development|PrintString 0 "ERROR! Could not find Armor Info!" true true "(R=0.615187,G=0.000000,B=1.000000,A=1.000000)" 4.0)))
  (return _returnvalue))