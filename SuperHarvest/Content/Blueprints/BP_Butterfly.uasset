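; BP_Butterfly is an ambient butterfly actor that flies between randomly chosen BP_Flower_Wild actors, or to a random point in its Box when none exist.
; After a random start delay, it turns toward the goal with a yaw correction for the mesh.
; A timeline lerps the mesh there with a vector-track offset and a randomized, distance-scaled play rate, then repeats after a pause.
; The construction script assigns a random material.
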(event Custom|FindNewGoal
  (bind _box (Variables|Default|GetBox))
  (bind (_origin _boxextent) (Collision|GetComponentBounds _box))
  ;[1 1 1] Picking a flower in the scene as a new goal
  (bind _outactors (Actor|GetAllActorsOfClass "/Game/Interactibles/Wild_plants/BP_Flower_Wild.BP_Flower_Wild_C"))
  (bind _output_get (Variables|Default|SetFlower_array _outactors))
  (if (== (Utilities|Array|Length _output_get) 0)
    (Variables|Default|SetGoalLocation (Math|Random|RandomPointinBoundingBox _origin _boxextent))
    (else
      (Variables|Default|SetChosenFlower (Math|Random|RandomIntegerinRange 0 (- (Utilities|Array|Length (Variables|Default|GetFlower_array)) 1)))
      (Variables|Default|SetGoalLocation (Math|Vector|MakeVector (.X (Math|Vector|BreakVector (Transformation|GetWorldLocation (Variables|/Game/Interactibles/BP_Base_Interactable.BP_Base_Interactable_C|GetInteractableMesh (Utilities|Array|Get(acopy) (Variables|Default|GetFlower_array) (Variables|Default|GetChosenFlower)))))) (.Y (Math|Vector|BreakVector (Transformation|GetWorldLocation (Variables|/Game/Interactibles/BP_Base_Interactable.BP_Base_Interactable_C|GetInteractableMesh (Utilities|Array|Get(acopy) (Variables|Default|GetFlower_array) (Variables|Default|GetChosenFlower)))))) (+ (.Z (Math|Vector|BreakVector (Transformation|GetWorldLocation (Variables|/Game/Interactibles/BP_Base_Interactable.BP_Base_Interactable_C|GetInteractableMesh (Utilities|Array|Get(acopy) (Variables|Default|GetFlower_array) (Variables|Default|GetChosenFlower)))))) 5e+01)))))
  ;[1 1 1] Setting start location and end location
  (Variables|Default|SetStartLocation (Transformation|GetWorldLocation (Variables|Default|GetSkeletalMesh)))
  (Transformation|SetActorRotation (Math|Rotator|MakeRotator (.Roll (Math|Rotator|BreakRotator (Math|Rotator|FindLookatRotation (Variables|Default|GetStartLocation) (Variables|Default|GetGoalLocation)))) (.Pitch (Math|Rotator|BreakRotator (Math|Rotator|FindLookatRotation (Variables|Default|GetStartLocation) (Variables|Default|GetGoalLocation)))) (+ (.Yaw (Math|Rotator|BreakRotator (Math|Rotator|FindLookatRotation (Variables|Default|GetStartLocation) (Variables|Default|GetGoalLocation)))) 9e+01)))
  ;[1 1 1] Set random speed for timeline
  (Variables|Default|SetRate 1.0)
  (Variables|Default|SetRate (+ (/ (Variables|Default|GetRate) (Math|Conversions|ToFloat(Integer) (+ (Math|Float|Round (/ (Math|Vector|VectorLength (- (Variables|Default|GetStartLocation) (Variables|Default|GetGoalLocation))) 1e+03)) 1))) (Math|Random|RandomFloatinRange 0.0 0.4)))
  (Components|Timeline|SetPlayRate (Variables|Default|GetGoToFlower) (Variables|Default|GetRate))
  ;[1 1 1] update butterly location by timeline
  (bind (_direction _alpha _vector_01) (Timeline|GoToFlower PlayFromStart)
    (:Update
      (Transformation|SetWorldLocation (Variables|Default|GetSkeletalMesh) (Math|Vector|Lerp(Vector) (Variables|Default|GetStartLocation) (+ _vector_01 (Variables|Default|GetGoalLocation)) _alpha) false false))
    (:Finished
      (Utilities|FlowControl|Delay 3.0)
      (CallFunction|FindNewGoal))))

(event EventBeginPlay
  (bind _box (Variables|Default|GetBox))
  (bind (_origin _boxextent) (Collision|GetComponentBounds _box))
  ;[1 1 1] Picking a flower in the scene as a new goal
  (Utilities|FlowControl|Delay (Math|Random|RandomFloatinRange 0.0 2.0))
  (bind _outactors (Actor|GetAllActorsOfClass "/Game/Interactibles/Wild_plants/BP_Flower_Wild.BP_Flower_Wild_C"))
  (bind _output_get (Variables|Default|SetFlower_array _outactors))
  (if (== (Utilities|Array|Length _output_get) 0)
    (Variables|Default|SetGoalLocation (Math|Random|RandomPointinBoundingBox _origin _boxextent))
    (else
      (Variables|Default|SetChosenFlower (Math|Random|RandomIntegerinRange 0 (- (Utilities|Array|Length (Variables|Default|GetFlower_array)) 1)))
      (Variables|Default|SetGoalLocation (Math|Vector|MakeVector (.X (Math|Vector|BreakVector (Transformation|GetWorldLocation (Variables|/Game/Interactibles/BP_Base_Interactable.BP_Base_Interactable_C|GetInteractableMesh (Utilities|Array|Get(acopy) (Variables|Default|GetFlower_array) (Variables|Default|GetChosenFlower)))))) (.Y (Math|Vector|BreakVector (Transformation|GetWorldLocation (Variables|/Game/Interactibles/BP_Base_Interactable.BP_Base_Interactable_C|GetInteractableMesh (Utilities|Array|Get(acopy) (Variables|Default|GetFlower_array) (Variables|Default|GetChosenFlower)))))) (+ (.Z (Math|Vector|BreakVector (Transformation|GetWorldLocation (Variables|/Game/Interactibles/BP_Base_Interactable.BP_Base_Interactable_C|GetInteractableMesh (Utilities|Array|Get(acopy) (Variables|Default|GetFlower_array) (Variables|Default|GetChosenFlower)))))) 5e+01)))))
  ;[1 1 1] Setting start location and end location
  (Variables|Default|SetStartLocation (Transformation|GetWorldLocation (Variables|Default|GetSkeletalMesh)))
  (Transformation|SetActorRotation (Math|Rotator|MakeRotator (.Roll (Math|Rotator|BreakRotator (Math|Rotator|FindLookatRotation (Variables|Default|GetStartLocation) (Variables|Default|GetGoalLocation)))) (.Pitch (Math|Rotator|BreakRotator (Math|Rotator|FindLookatRotation (Variables|Default|GetStartLocation) (Variables|Default|GetGoalLocation)))) (+ (.Yaw (Math|Rotator|BreakRotator (Math|Rotator|FindLookatRotation (Variables|Default|GetStartLocation) (Variables|Default|GetGoalLocation)))) 9e+01)))
  ;[1 1 1] Set random speed for timeline
  (Variables|Default|SetRate 1.0)
  (Variables|Default|SetRate (+ (/ (Variables|Default|GetRate) (Math|Conversions|ToFloat(Integer) (+ (Math|Float|Round (/ (Math|Vector|VectorLength (- (Variables|Default|GetStartLocation) (Variables|Default|GetGoalLocation))) 1e+03)) 1))) (Math|Random|RandomFloatinRange 0.0 0.4)))
  (Components|Timeline|SetPlayRate (Variables|Default|GetGoToFlower) (Variables|Default|GetRate))
  ;[1 1 1] update butterly location by timeline
  (bind (_direction _alpha _vector_01) (Timeline|GoToFlower PlayFromStart)
    (:Update
      (Transformation|SetWorldLocation (Variables|Default|GetSkeletalMesh) (Math|Vector|Lerp(Vector) (Variables|Default|GetStartLocation) (+ _vector_01 (Variables|Default|GetGoalLocation)) _alpha) false false))
    (:Finished
      (Utilities|FlowControl|Delay 3.0)
      (CallFunction|FindNewGoal))))

(fn ConstructionScript
  (Variables|Default|SetChosenInt (Math|Random|RandomIntegerinRange 0 2))
  (Rendering|Material|SetMaterial (Variables|Default|GetSkeletalMesh) 0 (Utilities|Array|Get(acopy) (Variables|Default|GetRandomMaterial) (Variables|Default|GetChosenInt)))
  (Rendering|Material|SetMaterial (Variables|Default|GetSkeletalMesh) 1 (Utilities|Array|Get(acopy) (Variables|Default|GetRandomMaterial) (Variables|Default|GetChosenInt))))