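; Soot melee enemy character that chases and attacks players behind a breakable, projectile-deflecting shield.
; A looping timer drives targeting, movement, attacks, and shield reactions to the player's facing and reloading.
; Damage also raises the shield, with timelines blending pose and walk speed, while shield hits drain durability and spawn return projectiles until it drops.
; Death ragdolls the body, detaches gear and rolls loot from a DataTable.
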(event OnComponentHit(ShieldCol)
  (params (HitComponent :type Primitive%20Component%20Object%20Reference) (OtherActor :type Actor%20Object%20Reference) (OtherComp :type Primitive%20Component%20Object%20Reference) (NormalImpulse :type Vector :default "0, 0, 0") (Hit :type Hit%20Result%20Structure%20%28by%20ref%29))
  (bind _self self)
  (bind _shield (Variables|Default|GetShield))
  (bind _shieldcol (Variables|Default|GetShieldCol))
  (bind _returnvalue (Math|Vector|GetForwardVector _shieldcol))
  (bind _returnvalue_2 (Transformation|GetWorldLocation _shieldcol))
  (bind _returnvalue_3 (* _returnvalue 2.0))
  (bind _returnvalue_4 (+ _returnvalue_2 _returnvalue_3))
  ;[1 1 1] Projectile Hit Shield?
  (if (Utilities|ClassIsChildOf (Utilities|GetClass OtherActor) "/Game/Blueprints/Projectiles/projectile_main.projectile_main_C")
    (Utilities|FlowControl|DoOnce false :!label _label
      (:Completed
        (Utilities|FlowControl|Sequence
          (:then_0
            (bind _output_get (Variables|Default|SetHitActor OtherActor))
            (bind _asprojectile_main (Utilities|Casting|CastToprojectile_main _output_get))
            (CallFunction|ShieldDamageVisibility)
            ;;[1 1 1] Shield Ruability loss on Shield Hit
            (Variables|Default|SetShieldDurability (- (Variables|Default|GetShieldDurability) (Variables|/Game/Blueprints/Projectiles/projectile_main.projectile_main_C|Getdamage _asprojectile_main)))
            (Rendering|Components|TextRender|SetText (Variables|Default|GetTextRender) (Utilities|Text|ToText(String) (Utilities|String|Append (Utilities|String|ToString(Integer) (Math|Float|Truncate (Variables|Default|GetShieldDurability))) "/" (Utilities|String|ToString(Integer) (Math|Float|Truncate (Variables|Default|GetStartShieldDurability))))))
            (Effects|SpawnEmitteratLocation "/Game/VFX/wood_chips_01.wood_chips_01" (Transformation|GetWorldLocation (Variables|Default|GetShieldCol)))
            (if (<= (Variables|Default|GetShieldDurability) 0.0)
              ;;[1 1 1] Drop Shield on Durability 0
              (Utilities|FlowControl|DoOnce false
                (:Completed
                  (Transformation|DetachFromComponent _shield "KeepWorld" "KeepWorld" "KeepWorld" true)
                  (Collision|SetCollisionEnabled _shield "PhysicsOnly")
                  (Physics|SetSimulatePhysics _shield true)
                  (CallFunction|FinalShieldDown)))
              (else
                ;;[1 1 1] Deflect bullets with shield
                (if (and (Utilities|ClassIsChildOf (Utilities|GetClass (Variables|Default|GetHitActor)) "/Game/Blueprints/Projectiles/projectile_main.projectile_main_C") (!= (Components|GetOwner (Variables|Default|GetHitActor)) self))
                  (Variables|Default|SetDeflected true)
                  (if (== (Variables|Default|GetShieldUp?) 0.0)
                    (Game|SpawnActorfromClass "/Game/Blueprints/Projectiles/EnemyProjectile.EnemyProjectile_C" (Math|Transform|MakeTransform _returnvalue_4 (Transformation|GetWorldRotation _shieldcol)) "AlwaysSpawn" _self 3.0 _self)
                    (else
                      (Game|SpawnActorfromClass "/Game/Blueprints/Projectiles/EnemyProjectile.EnemyProjectile_C" (Math|Transform|MakeTransform _returnvalue_4 (Transformation|GetWorldRotation (Variables|Collision|GetCapsuleComponent))) "AlwaysSpawn" _self 3.0 _self)))
                  (Utilities|FlowControl|Delay 0.1)
                  (Variables|Default|SetDeflected false)))))
          (:then_1
            (Utilities|FlowControl|Delay 0.1)
            (goto _label Reset)))))))

(event Custom|ShieldUp
  ;[1 1 1] Go Into Shield Stance on Damage + Enable Shield Colision
  (if (and (== (Variables|Default|GetShieldUp?) 0.0) (!= (Variables|Default|GetShieldDurability) 0.0))
    (Utilities|FlowControl|DoOnce false :!label _label
      (:Completed
        (bind _time (Timeline|lerpTime PlayFromStart)
          (:Update
            (Utilities|FlowControl|Sequence
              (:then_0
                (Variables|Default|SetShieldUp? (Math|Float|Lerp 0.0 1.0 _time)))
              (:then_1
                (Variables|/Script/Engine.CharacterMovementComponent|SetMaxWalkSpeed (Variables|Character|GetCharacterMovement) (Math|Float|Lerp (Variables|Default|GetStartRunSpeed) (Variables|Default|GetStartWalkSpeed) _time)))))
          (:Finished
            (Utilities|FlowControl|Sequence
              (:then_0
                (Utilities|FlowControl|RetriggerableDelay 1e+01)
                (if (Variables|Default|GetLooking%20At)
                  (CallFunction|ShieldDown)))
              (:then_1
                (goto _label Reset))
              (:then_2
                (Collision|SetCollisionEnabled (Variables|Default|GetShieldCol) "QueryOnly")))))))))

(event Custom|MainEvents
  (bind _topdowncharacterreference (Variables|Default|GetTopDownCharacterReference))
  (bind _topdowncharacterreference_2 (Variables|Default|GetTopDownCharacterReference))
  ;[1 1 1] AI
  (Utilities|FlowControl|Sequence
    (:then_0
      ;[1 1 1] Rotate HP Towards LOCAL Player Camera
      (Transformation|SetWorldRotation (Variables|Default|GetText) (Math|Rotator|FindLookatRotation (Transformation|GetWorldLocation (Variables|Default|GetText)) (Transformation|GetWorldLocation (Variables|/Game/Blueprints/TopDownCharacter.TopDownCharacter_C|GetCamera1 (.AsTop%20Down%20Character (Utilities|Casting|CastToTopDownCharacter (Game|GetPlayerCharacter 0)))))) false false))
    (:then_1
      ;[1 1 1] Select Target
      (if (== (Variables|Default|GetTopDownCharacterReference) 0)
        (bind _outactors (Actor|GetAllActorsOfClass "/Game/Blueprints/TopDownCharacter.TopDownCharacter_C"))
        (for _array_element _outactors
          (Variables|Default|SetCurrentDistanceTo (Transformation|GetDistanceTo _array_element self))
          (if (<= (Transformation|GetDistanceTo _array_element self) (Variables|Default|GetCurrentDistanceTo))
            (CallFunction|ServerSetTarget _array_element)))
        (elif (>= (Transformation|GetDistanceTo (Variables|Default|GetTopDownCharacterReference) self) 3e+02)
          (Utilities|FlowControl|DoOnce false :!label _label
            (:Completed
              (Development|PrintString "TOO FAR AWAY FOR AGGRO")
              (CallFunction|ServerUnSetTarget)))
          (else
            (goto _label Reset)))))
    (:then_2
      ;[1 1 1] MoveToActor
      (Utilities|IsValid _topdowncharacterreference_2
        (:Is%20Valid
          (if (not (<= (Transformation|GetDistanceTo _topdowncharacterreference_2) 1.5e+02))
            (CallFunction|ServerSetMove)))))
    (:then_3
      ;[1 1 1] Attack when within 100units. Wants to be moved to BlackBoard
      (Utilities|IsValid _topdowncharacterreference
        (:Is%20Valid
          (if (<= (Transformation|GetDistanceTo _topdowncharacterreference) 1e+02) :!label _label_2
            (Variables|Default|SetAttack true)
            (Utilities|FlowControl|Delay (Variables|Default|GetAttackAnimLength))
            (Variables|Default|SetAttack false)
            (goto _label_2)
            (else
              (Variables|Default|SetAttack false))))))
    (:then_4
      ;[1 1 1] Shield Up / Down on LookAt
      (Utilities|IsValid (Variables|Default|GetTopDownCharacterReference)
        (:Is%20Valid
          (if (and (>= (* (Math|Vector|DotProduct (Math|Vector|GetForwardVector (Math|Rotator|FindLookatRotation (Transformation|GetActorLocation) (Transformation|GetActorLocation (Variables|Default|GetTopDownCharacterReference)))) (Math|Vector|GetForwardVector (Transformation|GetWorldRotation (Variables|/Script/Engine.Character|GetCapsuleComponent (Variables|Default|GetTopDownCharacterReference))))) -1.0) 0.8) (!= (Variables|Default|GetShieldDurability) 0.0))
            (Utilities|FlowControl|DoOnce false :!label _label_3
              (:Completed
                (Variables|Default|SetLooking%20At true :!label _label_4)
                (CallFunction|ShieldUp)
                (goto _label_5 Reset)))
            (else
              (Utilities|FlowControl|DoOnce false :!label _label_5
                (:Completed
                  (Variables|Default|SetLooking%20At false :!label _label_6)
                  (CallFunction|ShieldDown)
                  (goto _label_3 Reset))))))))
    (:then_5
      ;[1 1 1] Shield Up / Down on Player Reload
      (Utilities|IsValid (Variables|Default|GetTopDownCharacterReference)
        (:Is%20Valid
          (if (!= (Variables|Default|GetShieldDurability) 0.0)
            (if (and (Variables|Default|GetLooking%20At) (Variables|/Game/Blueprints/TopDownCharacter.TopDownCharacter_C|GetReloading? (Variables|Default|GetTopDownCharacterReference)))
              (Utilities|FlowControl|Sequence
                (:then_0
                  (Utilities|FlowControl|DoOnce false :!label _label_7
                    (:Completed
                      (Utilities|FlowControl|Delay 0.5)
                      (goto _label_6))))
                (:then_1
                  (goto _label_8 Reset)))
              (else
                (Utilities|FlowControl|Sequence
                  (:then_0
                    (Utilities|FlowControl|DoOnce true :!label _label_8
                      (:Completed
                        (Utilities|FlowControl|Delay 0.5)
                        (goto _label_4))))
                  (:then_1
                    (goto _label_7 Reset)))))))))))

(event Custom|Final%20Shield%20Down
  ;[1 1 1] Go Into Shield Stance on Damage + Enable Shield Colision
  (Variables|Default|SetShieldUp? 0.0)
  (Variables|/Script/Engine.CharacterMovementComponent|SetMaxWalkSpeed (Variables|Character|GetCharacterMovement) 475.0))

(event Custom|ShieldDown
  ;[1 1 1] Go Into Shield Stance on Damage + Enable Shield Colision
  (if (!= (Variables|Default|GetShieldDurability) 0.0)
    (bind _time (Timeline|Timeline_0 PlayFromStart)
      (:Update
        (Utilities|FlowControl|Sequence
          (:then_0
            (Variables|Default|SetShieldUp? (Math|Float|Lerp 1.0 0.0 _time)))
          (:then_1
            (Variables|/Script/Engine.CharacterMovementComponent|SetMaxWalkSpeed (Variables|Character|GetCharacterMovement) (Math|Float|Lerp (Variables|Default|GetStartWalkSpeed) (Variables|Default|GetStartRunSpeed) _time)))
          (:then_2
            (Collision|SetCollisionEnabled (Variables|Default|GetShieldCol) "NoCollision")))))))

(event Custom|Shield%20Damage%20Visibility
  (bind _shield (Variables|Default|GetShield))
  ;[1 1 1] Damage Shader Toggle
  (Rendering|Material|SetMaterial _shield 0 "/Game/Assets/Materials/Emissive_Red.Emissive_Red")
  (Utilities|FlowControl|Delay 0.2)
  (Rendering|Material|SetMaterial _shield 0 (Variables|Default|GetShieldBaseColor)))

(event Custom|Server_SetTarget
  (params (TopDownCharacterReference :type Top%20Down%20Character%20Object%20Reference))
  ;[1 1 1] Select Target
  (Variables|Default|SetTopDownCharacterReference TopDownCharacterReference))

(event Custom|Soot%20Enemy%20Damage%20Visibility
  (bind _mesh (Variables|Character|GetMesh))
  ;[1 1 1] Damage Shader Toggle
  (Rendering|Material|SetMaterial _mesh 4 "/Game/Assets/Materials/Emissive_Red.Emissive_Red")
  (Utilities|FlowControl|Delay 0.15)
  (Rendering|Material|SetMaterial _mesh 4 (Variables|Default|GetSootBodyColor)))

(event Custom|Server_SetMove
  ;[1 1 1] MoveToActor
  (AI|Navigation|SimpleMovetoActor (AI|GetAIController self) (Variables|Default|GetTopDownCharacterReference)))

(event Custom|Server_UnSetTarget
  ;[1 1 1] Select Target
  (Variables|Default|SetTopDownCharacterReference 0))

(event EventBeginPlay
  ;[1 1 1] BeginPlay
  (Variables|Default|SetStartHealth (Variables|Default|GetHealth))
  (bind _output_get (Variables|Default|SetShieldDurability (* (Variables|Default|GetHealth) 1.0)))
  (Variables|Default|SetStartShieldDurability _output_get)
  (Variables|Default|SetStartRunSpeed (Variables|/Script/Engine.CharacterMovementComponent|GetMaxWalkSpeed (Variables|Character|GetCharacterMovement)))
  (Variables|Default|SetStartWalkSpeed 2e+02)
  (Variables|Default|SetSootBodyColor (Rendering|Material|GetMaterial (Variables|Character|GetMesh) 4))
  (Variables|Default|SetShieldBaseColor (Rendering|Material|GetMaterial (Variables|Default|GetShield) 0))
  (Utilities|Time|SetTimerbyEvent (delegate Custom|MainEvents) 0.5 true))

(event Game|Damage|EventAnyDamage
  (params (Damage :type Float%20%28single-precision%29) (DamageType :type Damage%20Type%20Object%20Reference) (InstigatedBy :type Controller%20Object%20Reference) (DamageCauser :type Actor%20Object%20Reference))
  (bind _sword (Variables|Default|GetSword))
  (bind _shield (Variables|Default|GetShield))
  ;[1 1 1] TakeDamage
  (Variables|Default|SetHealth (- (Variables|Default|GetHealth) Damage))
  (CallFunction|SootEnemyDamageVisibility)
  (if (<= (Variables|Default|GetHealth) 0.0)
    (Effects|SpawnEmitteratLocation "/Game/VFX/grass_straw_cloud_01.grass_straw_cloud_01" (Transformation|GetActorLocation))
    ;;[1 1 1] Death
    ;;;[1 1 1] Disable More! No Anim, No Ai
    (Pawn|Components|CharacterMovement|DisableMovement (Variables|Character|GetCharacterMovement))
    (Physics|SetSimulatePhysics (Variables|Character|GetMesh) true)
    (Rendering|Components|TextRender|SetText (Variables|Default|GetText) (Utilities|Text|ToText(String) (Utilities|String|Append "dead" "")))
    (Utilities|FlowControl|Sequence
      (:then_0
        (Transformation|DetachFromComponent _shield "KeepWorld" "KeepWorld" "KeepWorld" true)
        (Collision|SetCollisionEnabled _shield "PhysicsOnly")
        (Physics|SetSimulatePhysics _shield true))
      (:then_1
        (Transformation|DetachFromComponent _sword "KeepWorld" "KeepWorld" "KeepWorld" true)
        (Collision|SetCollisionEnabled _sword "PhysicsOnly")
        (Physics|SetSimulatePhysics _sword true))
      (:then_2
        (Components|Animation|SetAnimationMode (Variables|Character|GetMesh) "AnimationSingleNode"))
      (:then_3
        (Collision|SetCollisionEnabled (Variables|Collision|GetCapsuleComponent) "NoCollision"))
      (:then_4
        (CallFunction|SpawnLoot)))
    (else
      ;;[1 1 1] Set Shield Up on Damage
      (CallFunction|ShieldUp)
      ;;[1 1 1] Update HP Text
      (Effects|SpawnEmitteratLocation "/Game/VFX/leaf_fall_small.leaf_fall_small" (Transformation|GetActorLocation))
      (Rendering|Components|TextRender|SetText (Variables|Default|GetText) (Utilities|Text|ToText(String) (Utilities|String|Append (Utilities|String|ToString(Integer) (Math|Float|Truncate (Variables|Default|GetHealth))) "/" (Utilities|String|ToString(Integer) (Math|Float|Truncate (Variables|Default|GetStartHealth)))))))))

(fn ConstructionScript)

(fn SpawnLoot
  (bind _outrownames (DataTable|GetDataTableRowNames "/Game/Interactibles/Soot_LootList.Soot_LootList"))
  (for _array_element _outrownames
    (bind _returnvalue (Utilities|GetDataTableRow "/Game/Interactibles/Soot_LootList.Soot_LootList" _array_element)
      (:then
        (LocalVariables|SetDropChance (.DropChance (Utilities|Struct|BreakLootList _returnvalue)))
        (LocalVariables|SetIDName (.ID (Utilities|Struct|BreakLootList _returnvalue)))
        (LocalVariables|SetClassRef (.ActorClass (Utilities|Struct|BreakLootList _returnvalue)))
        (LocalVariables|SetMaxAmount (.MaxAmount (Utilities|Struct|BreakLootList _returnvalue)))
        (LocalVariables|SetMinAmount (.MinAmount (Utilities|Struct|BreakLootList _returnvalue)))
        (if (Math|Float|InRange(Float) (Math|Random|RandomFloatinRange 0.0 1.0) 0.0 (LocalVariables|GetDropChance))
          (for _index (range (LocalVariables|GetMinAmount) (LocalVariables|GetMaxAmount))
            (Game|SpawnActorfromClass (LocalVariables|GetClassRef) (Transformation|GetWorldTransform (Variables|Character|GetMesh)) "Undefined" 0 0))))
      (:RowNotFound
        (Development|PrintString "Error did not find row")))))