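; Spline-driven fence actor that builds a row of destructible fence pieces in the construction script.
; It divides the spline length by Spacing and adds a destructible component at each step, positioned and rotated to the spline in local space.
; The first piece uses FenceEnd, the last FenceStart, and those between pick an unseeded random mesh from the FenceRef array.
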(event EventBeginPlay)

(event Collision|EventActorBeginOverlap
  (params (OtherActor :type Actor%20Object%20Reference)))

(event EventTick
  (params (DeltaSeconds :type Float%20%28single-precision%29)))

(fn ConstructionScript
  (bind _spacing (Variables|Default|GetSpacing))
  (bind _fenceref (Variables|Default|GetFenceRef))
  (bind _spline (Variables|Default|GetSpline))
  (bind _returnvalue (Spline|GetSplineLength _spline))
  (bind _returnvalue_2 (Math|Float|Division(WholeandRemainder) _returnvalue _spacing))
  (for _index (range 0 _returnvalue_2)
    (bind _returnvalue_3 (AddComponent|AddDestructibleComponent false (Math|Transform|MakeTransform (Spline|GetLocationatDistanceAlongSpline _spline (* _index _spacing) "Local") (Spline|GetRotationatDistanceAlongSpline _spline (* _index _spacing) "Local"))))
    (if (== _index 0)
      (Variables|Default|SetDestrMeshRef (Variables|Default|GetFenceEnd))
      (elif (== _returnvalue_2 _index)
        (Variables|Default|SetDestrMeshRef (Variables|Default|GetFenceStart))
        (else
          (Variables|Default|SetDestrMeshRef (Utilities|Array|Get(acopy) _fenceref (Math|Random|RandomIntegerinRange 0 (- (Utilities|Array|Length _fenceref) 1)))))))
    (Class|DestructibleComponent|SetDestructibleMesh _returnvalue_3 (Variables|Default|GetDestrMeshRef))))