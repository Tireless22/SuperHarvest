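; Game instance Blueprint that hosts multiplayer lobbies and tears down sessions.
; CreateLobby stores the server settings, flags a real online game, and creates an Advanced Session advertising name, map, mode and LAN as extra settings.
; On success it opens the Lobby level as a listen server, while DestroySession ends the session for the first player controller.
; RepNotify handlers for the online flag and cosmetic player material are empty.
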(event Custom|CreateLobby
  (params (ServerName :type String) (ServerMap :type String) (ServerSlots :type Integer) (ServerMode :type String) (ServerMethod :type Boolean))
  ;[1 1 1] Create Lobby
  (Variables|Default|SetServerName ServerName)
  (Variables|Default|SetServerMap ServerMap)
  (Variables|Default|SetServerSlots ServerSlots)
  (Variables|Default|SetServerMode ServerMode)
  (Variables|Default|SetServerMethod ServerMethod)
  (Variables|Default|SetIsRealOnlineGame? true)
  (|AdvancedSession (Utilities|Array|MakeArray (Class|AdvancedSessionsLibrary|MakeLiteralSessionPropertyString "NAME" (Variables|Default|GetServerName)) (Class|AdvancedSessionsLibrary|MakeLiteralSessionPropertyString "MAP" (Variables|Default|GetServerMap)) (Class|AdvancedSessionsLibrary|MakeLiteralSessionPropertyString "MODE" (Variables|Default|GetServerMode)) (Class|AdvancedSessionsLibrary|MakeLiteralSessionPropertyBool "LAN" (Variables|Default|GetServerMethod))) (Game|GetPlayerController 0) (Variables|Default|GetServerSlots) 0 (Variables|Default|GetServerMethod) true false true true false false false true
    (:OnSuccess
      (Game|OpenLevel(byName) "Lobby" true "listen"))))

(event Custom|DestroySession
  ;[1 1 1] Destroy Session
  (|DestroySession (Game|GetPlayerController 0)))

(fn OnRepIsRealOnlineGame?)

(fn OnRepCosmeticPlayerMaterial)