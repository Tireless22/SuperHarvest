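; Weather and day/night manager that drives sun, skydome, skylight, optional fog and random rain.
; A looping timer at the clock widget's game speed advances time and samples curves for lighting, restarting when speed doubles or halves.
; A per-second roll starts timed rain with player-relative emitters, puddles, crossfaded ambience, sun tint and intensity fade, then a cooldown.
; The lightning logic is present but unconnected.
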(event Custom|SpawnInPuddles
  ;[1 1 1] spawn puddles
  (Variables|Default|SetNumberOfPuddles (Math|Random|RandomIntegerinRange 10 50))
  (for _index (range 0 (Variables|Default|GetNumberOfPuddles))
    (bind _returnvalue (Game|SpawnActorfromClass "/Game/Blueprints/WaterPuddle.WaterPuddle_C" (Math|Transform|MakeTransform (Math|Random|RandomPointinBoundingBox (Variables|Default|GetOrigo) (Variables|Default|GetBoxExtent)) (Math|Rotator|MakeRotator 0.0 0.0 (Math|Random|RandomFloatinRange 0.0 3.6e+02)) "1.000000,1.000000,1.000000") "Undefined" 0 0))
    (Utilities|Array|Add (Variables|Default|GetPuddleArray) _returnvalue)))

(event Custom|StartSunAndFog
  ;[1 1 1] update seconds passed
  (Variables|Default|SetSecondsPassed (+ (Variables|Default|GetSecondsPassed) 1.0))
  (Variables|Default|SetAlpha (/ (Variables|Default|GetSecondsPassed) (Variables|Default|GetDayTimeInSeconds)))
  ;[1 1 1] set fog density
  (CallFunction|SetFogDensity)
  ;[1 1 1] Update Sun Rotation
  (Transformation|SetActorRotation (Variables|ReferenceActors|GetSun) (Math|Rotator|MakeRotator 0.0 (Math|Curves|GetFloatValue (Variables|Curves|GetSunDirection) (* (Variables|Default|GetAlpha) (Variables|Default|GetDayTimeInSeconds))) (Math|Curves|GetFloatValue (Variables|Curves|GetSunDirectionZ) (* (Variables|Default|GetAlpha) (Variables|Default|GetDayTimeInSeconds)))))
  ;[1 1 1] set sun intensity
  (if (<= (- (* (Variables|Default|GetAlpha) (Variables|Default|GetDayTimeInSeconds)) (Variables|Default|GetFadeSunModifier)) 0.0)
    (Variables|Default|SetSunIntensity 0.0)
    (else
      (Variables|Default|SetSunIntensity (- (* (Variables|Default|GetAlpha) (Variables|Default|GetDayTimeInSeconds)) (Variables|Default|GetFadeSunModifier)))))
  (Rendering|Components|Light|SetIntensity (Variables|/Script/Engine.Light|GetLightComponent (Variables|ReferenceActors|GetSun)) (Math|Curves|GetFloatValue (Variables|Curves|GetSunIntensityCurve) (Variables|Default|GetSunIntensity)))
  ;[1 1 1] update skydome sun direction
  (Default|UpdateSunDirection (Variables|ReferenceActors|GetSkydome))
  ;[1 1 1] update indirect lighting intensity
  (Class|LightComponent|SetIndirectLightingIntensity (Variables|/Script/Engine.Light|GetLightComponent (Variables|ReferenceActors|GetSun)) (Math|Curves|GetFloatValue (Variables|Curves|GetIndirectLightingIntensity) (* (Variables|Default|GetAlpha) (Variables|Default|GetDayTimeInSeconds))))
  ;[1 1 1] evening fade skylight
  (Rendering|Components|Light|SetIntensity (Variables|/Script/Engine.SkyLight|GetLightComponent (Variables|ReferenceActors|GetSkyLight)) (Math|Curves|GetFloatValue (Variables|Curves|GetSkylightIntensity) (* (Variables|Default|GetAlpha) (Variables|Default|GetDayTimeInSeconds)))))

(event Custom|RestartWeather
  ;[1 1 1] restart weather
  (Variables|Default|SetSunAngle 0.0)
  (Variables|Default|SetSecondsPassed 0.0)
  (Variables|Default|SetIndirectIntensity 1.0)
  (Variables|Default|SetFogDistanceSet? true)
  (Variables|Default|SetCurrentLocation "0, 0, 0")
  (Variables|Default|SetRainLooping? false)
  (Variables|Default|SetRainDuration 0.0)
  (Variables|Default|SetRainDestroyed? true)
  (Variables|Default|SetSpawnZHeight 6.2e+02)
  (Variables|Default|SetChanceForRainPerSecond 1)
  (Variables|Default|SetChanceForLightning 100)
  (Variables|Default|SetLightning? false)
  (Utilities|Array|Clear (Variables|Default|GetLightningLocationArray))
  (Variables|Default|SetMaxNrLightningStrikes 1)
  (Variables|Default|SetRainCooldown 1e+01)
  (Variables|Default|SetChosenInt 0)
  (Variables|Default|SetCurrentTime 0.0)
  (Variables|Default|SetFadeSunModifier 3.0)
  (Variables|Default|SetRainMaxDuration 25.0)
  (Variables|Default|SetSkyLightDefaultIntensity 2.0)
  (Variables|Default|SetSkylightNightIntensity 0.5)
  (Variables|Default|SetSkyLightCurrentIntensity 2.0)
  (Variables|Default|SetSecondsCounter 0.0)
  (Variables|Default|SetGameTimeSpeedRef 0.0)
  (Variables|Default|SetAlpha 0.0)
  (Variables|Default|SetDayTimeInSeconds 1.2e+03)
  (Variables|Default|SetFogEnabled? false)
  ;[1 1 1] Get Game Time Speed
  (bind _foundwidgets (Widget|GetAllWidgetsOfClass "/Game/UI/UI_Clock.UI_Clock_C" false))
  (Utilities|IsValid (Utilities|Array|Get(acopy) _foundwidgets)
    (:Is%20Valid
      (bind _asui_clock (Utilities|Casting|CastToUI_Clock (Utilities|Array|Get(acopy) _foundwidgets))
        (:then
          (Variables|Default|SetGameTimeSpeedRef (Variables|/Game/UI/UI_Clock.UI_Clock_C|GetGameTimeSpeed _asui_clock))
          ;[1 1 1] start forest sound
          (bind _returnvalue (CallFunction|SpawnSoundAttached "/Game/SFX/cue_forest_loop.cue_forest_loop"))
          (Variables|Default|SetForestSoundRef _returnvalue)
          ;[1 1 1] start weather
          (Utilities|Time|SetTimerbyEvent (delegate Custom|WeatherInitiator) 1.0 true)
          ;[1 1 1] Start update sun and fog
          (bind _returnvalue_2 (Utilities|Time|SetTimerbyEvent (delegate Custom|StartSunAndFog) (Variables|Default|GetGameTimeSpeedRef) true)))
        (:CastFailed
          (Development|PrintString "castfail233"))))
    (:Is%20Not%20Valid
      (Development|PrintString "not valid"))))

(event Custom|StartRain
  (Development|PrintString "Rain Started!")
  (Variables|Default|SetRainDestroyed? false)
  (Variables|Default|SetRainDuration (Math|Random|RandomFloatinRange 15.0 (Variables|Default|GetRainMaxDuration)))
  (Variables|Default|SetCurrentTime 0.0)
  (Utilities|FlowControl|Sequence
    (:then_0
      ;[1 1 1] rain event
      (if (>= (Variables|Default|GetSecondsCounter) 7.8e+02)
        _
        (else
          (bind _returnvalue (Utilities|Time|SetTimerbyEvent (delegate Custom|FadeSun) 0.1 true))
          (Variables|Default|SetFadeSunHandle _returnvalue)))
      (bind _returnvalue_2 (Utilities|Time|SetTimerbyEvent (delegate Custom|RainVFX) 1.0 true))
      (Variables|Default|SetRainVFXHandle _returnvalue_2)
      (CallFunction|RainTimer)
      (CallFunction|StartRainSound)
      (CallFunction|SpawninPuddles))
    (:then_1
      ;[1 1 1] Lerp Color on start
      (bind _alpha (Timeline|ColorLerpStart PlayFromStart)
        (:Update
          (Rendering|Components|Light|SetLightColor (Variables|/Script/Engine.Light|GetLightComponent (Variables|ReferenceActors|GetSun)) (Math|Color|Lerp(LinearColor) "(R=1.000000,G=1.000000,B=1.000000,A=1.000000)" "(R=0.305100,G=0.424356,B=0.540000,A=1.000000)" _alpha) true))))))

(event Custom|FadeSun
  ;[1 1 1] FadeSun
  (Variables|Default|SetCurrentTime (+ (Variables|Default|GetCurrentTime) 0.1))
  (if (< (Variables|Default|GetCurrentTime) (Variables|Default|GetRainDuration))
    (if (not (<= (Variables|Default|GetFadeSunModifier) -1.5))
      (Variables|Default|SetFadeSunModifier (- (Variables|Default|GetFadeSunModifier) 0.1)))
    (elif (>= (Variables|Default|GetFadeSunModifier) 0.0)
      (Variables|Default|SetFadeSunModifier 0.0)
      (Utilities|Time|ClearandInvalidateTimerbyHandle (Variables|Default|GetFadeSunHandle))
      (else
        (Variables|Default|SetFadeSunModifier (+ (Variables|Default|GetFadeSunModifier) 0.1))))))

(event Custom|RainTimer
  ;[1 1 1] On rain end
  (Utilities|FlowControl|Delay (Variables|Default|GetRainDuration))
  (Utilities|FlowControl|Sequence
    (:then_0
      ;[1 1 1] Lerp sun color
      (bind _alpha (Timeline|ColorLerpEnd PlayFromStart)
        (:Update
          (Rendering|Components|Light|SetLightColor (Variables|/Script/Engine.Light|GetLightComponent (Variables|ReferenceActors|GetSun)) (Math|Color|Lerp(LinearColor) "(R=0.304987,G=0.423268,B=0.539480,A=1.000000)" "(R=1.000000,G=1.000000,B=1.000000,A=1.000000)" _alpha) true))))
    (:then_1
      ;[1 1 1] Fade out Rain sound
      (Audio|Components|Audio|FadeOut (Variables|Default|GetRainSoundRef) 2.9 0.0 :!class /Script/Engine.AudioComponent)
      ;[1 1 1] invalidate timer
      (Utilities|FlowControl|Delay 2.0)
      (Utilities|Time|ClearandInvalidateTimerbyHandle (Variables|Default|GetRainVFXHandle))
      ;[1 1 1] reset rain destroyed after cooldown
      (Utilities|FlowControl|Delay (Variables|Default|GetRainCooldown))
      (Variables|Default|SetRainDestroyed? true))
    (:then_2
      ;[1 1 1] Fade in forest sound
      (Utilities|FlowControl|Delay 2.0)
      (bind _returnvalue (CallFunction|SpawnSoundAttached "/Game/SFX/cue_forest_loop.cue_forest_loop"))
      (Variables|Default|SetForestSoundRef _returnvalue)
      (Audio|Components|Audio|FadeIn (Variables|Default|GetForestSoundRef) 2.0 1.0 0.0 :!class /Script/Engine.AudioComponent))
    (:then_3
      ;[1 1 1] fade out puddles
      (Utilities|FlowControl|Delay 3.0)
      (for _array_element (Variables|Default|GetPuddleArray)
        (Default|FadeOutPuddle _array_element))
      (Utilities|Array|Clear (Variables|Default|GetPuddleArray)))))

(event Custom|RefreshSunFogTimer
  (Utilities|Time|ClearandInvalidateTimerbyHandle (stale _returnvalue))
  ;[1 1 1] Start update sun and fog
  (bind _returnvalue (Utilities|Time|SetTimerbyEvent (delegate Custom|StartSunAndFog) (Variables|Default|GetGameTimeSpeedRef) true)))

(event Custom|StartRainSound
  (bind _forestsoundref (Variables|Default|GetForestSoundRef))
  ;[1 1 1] start rain sound
  (Utilities|FlowControl|Delay 1.0)
  (bind _returnvalue (CallFunction|SpawnSoundAttached "/Game/SFX/cue_rain_loop.cue_rain_loop"))
  (Variables|Default|SetRainSoundRef _returnvalue)
  (Audio|Components|Audio|FadeIn (Variables|Default|GetRainSoundRef) 2.0 1.0 0.0 :!class /Script/Engine.AudioComponent)
  (Utilities|IsValid _forestsoundref
    (:Is%20Valid
      (Audio|Components|Audio|FadeOut _forestsoundref 2.0 0.0 :!class /Script/Engine.AudioComponent))))

(event Custom|RainVFX
  ;[1 1 1] rain event
  (bind _astop_down_character (Utilities|Casting|CastToTopDownCharacter (Game|GetPlayerCharacter 0)))
  (Variables|Default|SetCurrentLocation (Transformation|GetWorldLocation (Variables|/Script/Engine.Character|GetMesh _astop_down_character)))
  (Utilities|FlowControl|Sequence
    (:then_0
      (Effects|SpawnEmitteratLocation "/Game/Assets/VFX/Rain_Hit_Ground.Rain_Hit_Ground" (Math|Vector|MakeVector (+ (.X (Math|Vector|BreakVector (Variables|Default|GetCurrentLocation))) 7e+02) (+ (.Y (Math|Vector|BreakVector (Variables|Default|GetCurrentLocation))) 1e+03) (Variables|Default|GetSpawnZHeight))))
    (:then_1
      (Effects|SpawnEmitteratLocation "/Game/Assets/VFX/Rain_Hit_Ground.Rain_Hit_Ground" (Math|Vector|MakeVector (+ (.X (Math|Vector|BreakVector (Variables|Default|GetCurrentLocation))) 7e+02) (- (.Y (Math|Vector|BreakVector (Variables|Default|GetCurrentLocation))) 1e+03) (Variables|Default|GetSpawnZHeight))))
    (:then_2
      (Effects|SpawnEmitteratLocation "/Game/Assets/VFX/Rain_Hit_Ground.Rain_Hit_Ground" (Math|Vector|MakeVector (- (.X (Math|Vector|BreakVector (Variables|Default|GetCurrentLocation))) 7e+02) (+ (.Y (Math|Vector|BreakVector (Variables|Default|GetCurrentLocation))) 1e+03) (Variables|Default|GetSpawnZHeight))))
    (:then_3
      (Effects|SpawnEmitteratLocation "/Game/Assets/VFX/Rain_Hit_Ground.Rain_Hit_Ground" (Math|Vector|MakeVector (- (.X (Math|Vector|BreakVector (Variables|Default|GetCurrentLocation))) 7e+02) (- (.Y (Math|Vector|BreakVector (Variables|Default|GetCurrentLocation))) 1e+03) (Variables|Default|GetSpawnZHeight))))))

(event Custom|WeatherInitiator
  ;[1 1 1] Roll for Rain
  (if (Variables|Default|GetRainDestroyed?)
    (bind __ (CallFunction|Percentage (Variables|Default|GetChanceForRainPerSecond)))
    (if __
      (CallFunction|StartRain))))

(event EventBeginPlay
  ;[1 1 1] Event begin play
  ;[1 1 1] Get Game Time Speed
  (bind _foundwidgets (Widget|GetAllWidgetsOfClass "/Game/UI/UI_Clock.UI_Clock_C" false))
  (Utilities|IsValid (Utilities|Array|Get(acopy) _foundwidgets)
    (:Is%20Valid
      (bind _asui_clock (Utilities|Casting|CastToUI_Clock (Utilities|Array|Get(acopy) _foundwidgets))
        (:then
          (Variables|Default|SetGameTimeSpeedRef (Variables|/Game/UI/UI_Clock.UI_Clock_C|GetGameTimeSpeed _asui_clock))
          ;[1 1 1] start forest sound
          (bind _returnvalue (CallFunction|SpawnSoundAttached "/Game/SFX/cue_forest_loop.cue_forest_loop"))
          (Variables|Default|SetForestSoundRef _returnvalue)
          ;[1 1 1] start weather
          (Utilities|Time|SetTimerbyEvent (delegate Custom|WeatherInitiator) 1.0 true)
          ;[1 1 1] Start update sun and fog
          (bind _returnvalue_2 (Utilities|Time|SetTimerbyEvent (delegate Custom|StartSunAndFog) (Variables|Default|GetGameTimeSpeedRef) true)))
        (:CastFailed
          (Development|PrintString "castfail233"))))
    (:Is%20Not%20Valid
      (Development|PrintString "not valid"))))

(event EventDoubleSpeed
  ;[1 1 1] Event global time change
  (if (not (<= (Variables|Default|GetGameTimeSpeedRef) 0.025))
    (Variables|Default|SetGameTimeSpeedRef (/ (Variables|Default|GetGameTimeSpeedRef) 2.0))
    (CallFunction|RefreshSunFogTimer)))

(event EventSetTime
  (params (NewTimeInHours :type Float%20%28single-precision%29))
  ;[1 1 1] Event global time change
  (if (Math|Float|InRange(Float) NewTimeInHours 0.0 26.0)
    (Variables|Default|SetSecondsPassed (* (- NewTimeInHours 6.0) 6e+01))))

(event EventHalfSpeed
  ;[1 1 1] Event global time change
  (if (not (>= (Variables|Default|GetGameTimeSpeedRef) 0.4))
    (Variables|Default|SetGameTimeSpeedRef (* (Variables|Default|GetGameTimeSpeedRef) 2.0))
    (CallFunction|RefreshSunFogTimer)))

(fn ConstructionScript)

(fn SpawnSoundAttached
  (params (sound :type Sound%20Base%20Object%20Reference))
  (bind _astop_down_character (Utilities|Casting|CastToTopDownCharacter (Game|GetPlayerCharacter 0))
    (:then
      (bind _returnvalue (Audio|SpawnSoundAttached sound (Variables|/Script/Engine.Character|GetMesh _astop_down_character) "MainChar_Root"))
      (return _returnvalue))
    (:CastFailed
      (Development|PrintString "cast fail"))))

(fn SetFogDensity
  (if (Variables|Default|GetFogEnabled?)
    (Class|ExponentialHeightFogComponent|SetFogDensity (Variables|Default|GetExponentialHeightFog) (Math|Curves|GetFloatValue (Variables|Curves|GetFogDensity) (* (Variables|Default|GetAlpha) (Variables|Default|GetDayTimeInSeconds)))))
  (return))