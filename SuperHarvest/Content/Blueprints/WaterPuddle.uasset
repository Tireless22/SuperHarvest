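; Water puddle actor that gradually fades into view on spawn and fades away before destroying itself.
; On BeginPlay it creates a dynamic cut-fade water material on the puddle mesh and starts a looping timer that steps the inverted Alpha parameter down from fully faded.
; FadeOutPuddle starts a second timer that steps Alpha back up, then destroys the actor once it is fully faded.
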(event Custom|StartFadeIn
  ;[1 1 1] fade in
  (Variables|Default|SetAlpha (- (Variables|Default|GetAlpha) (Variables|Default|GetValueToChange)))
  (if (<= (Variables|Default|GetAlpha) (Variables|Default|GetValueToChange))
    (Rendering|Material|SetScalarParameterValue (Variables|Default|GetMaterialRef) "Alpha" (Variables|Default|GetValueToChange) :!class /Script/Engine.MaterialInstanceDynamic)
    (Utilities|Time|ClearandInvalidateTimerbyHandle (stale EventBeginPlay _returnvalue_2))
    (else
      (Rendering|Material|SetScalarParameterValue (Variables|Default|GetMaterialRef) "Alpha" (Variables|Default|GetAlpha) :!class /Script/Engine.MaterialInstanceDynamic))))

(event Custom|FadeOutPuddle
  ;[1 1 1] fade out
  (bind _returnvalue (Utilities|Time|SetTimerbyEvent (delegate Custom|StartFadeOut) 0.2 true)))

(event Custom|StartFadeOut
  ;[1 1 1] fade out
  (Variables|Default|SetAlpha (+ (Variables|Default|GetAlpha) (Variables|Default|GetValueToChange)))
  (if (>= (Variables|Default|GetAlpha) 1.0)
    (Rendering|Material|SetScalarParameterValue (Variables|Default|GetMaterialRef) "Alpha" 1.0 :!class /Script/Engine.MaterialInstanceDynamic)
    (Utilities|Time|ClearandInvalidateTimerbyHandle (stale Custom|FadeOutPuddle _returnvalue))
    (Actor|DestroyActor)
    (else
      (Rendering|Material|SetScalarParameterValue (Variables|Default|GetMaterialRef) "Alpha" (Variables|Default|GetAlpha) :!class /Script/Engine.MaterialInstanceDynamic))))

(event EventBeginPlay
  ;[1 1 1] create dyn material
  (bind _returnvalue (Rendering|Material|CreateDynamicMaterialInstance (Variables|Default|GetPuddleMesh) 0 "/Game/Assets/VFX/Materials/CutFadeMaterial_Inst3_water.CutFadeMaterial_Inst3_water" :!class /Script/Engine.PrimitiveComponent))
  (Variables|Default|SetMaterialRef _returnvalue)
  (Rendering|Material|SetScalarParameterValue (Variables|Default|GetMaterialRef) "Alpha" 1.0 :!class /Script/Engine.MaterialInstanceDynamic)
  (Variables|Default|SetAlpha 1.0)
  (Variables|Default|SetValueToChange (/ (+ 0.0 0.5) 32.0))
  ;[1 1 1] fade in
  (bind _returnvalue_2 (Utilities|Time|SetTimerbyEvent (delegate Custom|StartFadeIn) 0.2 true)))

(fn ConstructionScript)